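; BP_Casher is a collection zone that banks the score of balls touching it.
; When a BP_Ball_Base overlaps CasherCollision, it adds the ball's current score to the global score through the MT game state, then unregisters and destroys the ball.
; Once all balls are destroyed, it waits briefly and switches the game state to round end.
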(event `self.CasherCollision.OnComponentBeginOverlap`
  (params (OverlappedComponent :type "PrimitiveComponent Object Reference") (OtherActor :type "Actor Object Reference") (OtherComp :type "PrimitiveComponent Object Reference") (OtherBodyIndex :type Integer) (bFromSweep :type Boolean) (SweepResult :type "HitResult Structure (by ref)"))
  (bind _asbp_ball_base (cast `/Game/Core/Ingredients/Balls/BP_Ball_Base` OtherActor))
  (`/Game/Core/Game/BP_GameState.UpdateGlobalScore` (`/Game/Core/Common/Helpers/BFL_Getters.GetMTGameState`) (`/Game/Core/Ingredients/Balls/BP_Ball_Base.CurrentScore` _asbp_ball_base))
  (`/Game/Core/Game/BP_GameState.RemoveSpawnedBall` (`/Game/Core/Common/Helpers/BFL_Getters.GetMTGameState`) _asbp_ball_base)
  (`self.K2_DestroyActor` _asbp_ball_base)
  (if (`/Game/Core/Game/BP_GameState.AreAllBallsDestroyed` (`/Game/Core/Common/Helpers/BFL_Getters.GetMTGameState`))
    (`KismetSystemLibrary.Delay` 2.0)
    (`/Game/Core/Game/BP_GameState.ChangeState` (`/Game/Core/Common/Helpers/BFL_Getters.GetMTGameState`) "/Game/Core/Game/States/BPC_GameState_GB_RoundEnd.BPC_GameState_GB_RoundEnd_C")))

(fn `UserConstructionScript`)