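; Homunculus ingredient actor that the player can highlight on hover and pick up by clicking while in the Wandering state.
; Clicking clears the outline overlay, sets the player's point light intensity, switches the player to Lifting and registers itself as the lifted object.
; While lifted, Tick teleports the mesh ahead of the player, facing them, and prints its target position.
; On hit, the mesh stops simulating physics and yaws toward the player.
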(event `/Game/Core/Common/Interfaces/BPI_ClickableObject.OnClickStart`
  (if (== (`/Game/Core/Player/BP_PlayerCharacter.CurrentState` (`/Game/Core/Common/Helpers/BFL_Getters.GetMTPlayerCharacter`)) "/Game/Core/Player/States/BPC_PlayerState_Wandering.BPC_PlayerState_Wandering_C")
    (if (not (`self.IsBeingLifted`))
      (set `self.IsBeingLifted` true)
      (`MeshComponent.SetOverlayMaterial` (`self.SM_Homon`) null)
      (`LightComponent.SetIntensity` (`/Game/Core/Player/BP_PlayerCharacter.PointLight` (`/Game/Core/Common/Helpers/BFL_Getters.GetMTPlayerCharacter`)) 25.0)
      (`/Game/Core/Player/BP_PlayerCharacter.ChangeState` (`/Game/Core/Common/Helpers/BFL_Getters.GetMTPlayerCharacter`) "/Game/Core/Player/States/BPC_PlayerState_Lifting.BPC_PlayerState_Lifting_C")
      (set `/Game/Core/Player/BP_PlayerCharacter.LiftedObject` self (`/Game/Core/Common/Helpers/BFL_Getters.GetMTPlayerCharacter`)))))

(event `/Game/Core/Common/Interfaces/BPI_ClickableObject.OnHoveredStart`
  (if (== (`/Game/Core/Player/BP_PlayerCharacter.CurrentState` (`/Game/Core/Common/Helpers/BFL_Getters.GetMTPlayerCharacter`)) "/Game/Core/Player/States/BPC_PlayerState_Wandering.BPC_PlayerState_Wandering_C")
    (`MeshComponent.SetOverlayMaterial` (`self.SM_Homon`) "/Game/Materials/M_Outline.M_Outline")))

(event `/Game/Core/Common/Interfaces/BPI_ClickableObject.OnHoveredEnd`
  (if (== (`/Game/Core/Player/BP_PlayerCharacter.CurrentState` (`/Game/Core/Common/Helpers/BFL_Getters.GetMTPlayerCharacter`)) "/Game/Core/Player/States/BPC_PlayerState_Wandering.BPC_PlayerState_Wandering_C")
    (`MeshComponent.SetOverlayMaterial` (`self.SM_Homon`) null)))

(event `self.ReceiveTick`
  (params (DeltaSeconds :type "Float (single-precision)"))
  (bind _mtplayercharacter (`/Game/Core/Common/Helpers/BFL_Getters.GetMTPlayerCharacter`))
  (bind _returnvalue (`self.K2_GetActorLocation` _mtplayercharacter))
  (bind (_returnvalue_roll _returnvalue_pitch _returnvalue_yaw) (`KismetMathLibrary.BreakRotator` (`KismetMathLibrary.FindLookAtRotation` (`SceneComponent.K2_GetComponentLocation` (`self.SM_Homon`)) _returnvalue)))
  (bind _returnvalue_2 (+ _returnvalue (* (`self.GetActorForwardVector` _mtplayercharacter) 200.0)))
  (if (`self.IsBeingLifted`)
    (`KismetSystemLibrary.PrintString` (`KismetStringLibrary.Conv_VectorToString` _returnvalue_2))
    (`SceneComponent.K2_SetWorldLocation` (`self.SM_Homon`) _returnvalue_2 false true)
    (`SceneComponent.K2_SetWorldRotation` (`self.SM_Homon`) (`KismetMathLibrary.MakeRotator` _returnvalue_roll _returnvalue_pitch _returnvalue_yaw) false false)))

(event `self.SM_Homon.OnComponentHit`
  (params (HitComponent :type "PrimitiveComponent Object Reference") (OtherActor :type "Actor Object Reference") (OtherComp :type "PrimitiveComponent Object Reference") (NormalImpulse :type "Vector Structure") (Hit :type "HitResult Structure (by ref)"))
  (bind (_returnvalue_roll _returnvalue_pitch _returnvalue_yaw) (`KismetMathLibrary.BreakRotator` (`KismetMathLibrary.FindLookAtRotation` (`SceneComponent.K2_GetComponentLocation` (`self.SM_Homon`)) (`self.K2_GetActorLocation` (`/Game/Core/Common/Helpers/BFL_Getters.GetMTPlayerCharacter`)))))
  (`PrimitiveComponent.SetSimulatePhysics` (`self.SM_Homon`) false)
  (`SceneComponent.K2_SetWorldRotation` (`self.SM_Homon`) (`KismetMathLibrary.MakeRotator` 0.0 0.0 _returnvalue_yaw) false true))

(fn `UserConstructionScript`)