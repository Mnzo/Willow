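; Combinations note actor that stays pinned to the camera's left, nudges on hover, and on click zooms to screen center, hiding the main UI stack.
; While centered it tilts with the mouse, and timelines drive the hover and center moves and their reversal.
; When the player holds a dice combination and inputs are active, it gets an outline overlay and a looping random roll wiggle.
; A dynamic material dims it while inputs are disabled.
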(event `self.ReceiveBeginPlay`
  (add `/Game/Core/Player/BP_PlayerController_Game.OnInputsActivationToggled` (`/Game/Core/Common/Helpers/BFL_Getters.GetMTGameController`) (`|CreateDelegate` :!event `OnInputsActivationToggled`))
  (bind _returnvalue (`KismetMaterialLibrary.CreateDynamicMaterialInstance` "/Game/Assets/3D/Environment/Materials/M_Note2.M_Note2"))
  (set `self.DMI_Note` _returnvalue)
  (`PrimitiveComponent.SetMaterial` (`self.SM_CombinationsNote`) 0 (`self.DMI_Note`))
  (add `/Game/Core/Player/BP_PlayerCharacter.OnCurrentCombinationChanged` (`/Game/Core/Common/Helpers/BFL_Getters.GetMTPlayerCharacter`) (`|CreateDelegate` :!event `OnCurrentCombinationsChanged`))
  (set `self.InitialRotation` (`SceneComponent.RelativeRotation` (`self.SM_CombinationsNote`))))

(event `self.ReceiveTick`
  (params (DeltaSeconds :type "Float (single-precision)"))
  (bind (_cameralocation _camerarotation _cameraforwardvector _camerarightvector) (`/Game/Core/Player/BP_BasePlayerController.GetCurrentCameraData` (`/Game/Core/Common/Helpers/BFL_Getters.GetMTGameController`)))
  (if (`self.IsAttached`)
    (`self.K2_SetActorLocation` (+ _cameralocation (* _cameraforwardvector 200.0) (* _camerarightvector -295.0)))
    (`self.K2_SetActorRotation` (`KismetMathLibrary.MakeRotFromX` _cameraforwardvector))
    (elif (`self.IsCentered`)
      (`self.ProcessTiltBehavior`))))

(event `/Game/Core/Common/Interfaces/BPI_ClickableObject.OnClickStart`
  (if (not (`self.IsCentered`))
    (set `self.IsAttached` false)
    (set `self.IsCentered` true)
    (`self.PlayCenterTimeline`)
    (`/Game/Core/Player/BP_PlayerCharacter.ChangeState` (`/Game/Core/Common/Helpers/BFL_Getters.GetMTPlayerCharacter`) "/Game/Core/Player/States/BPC_PlayerState_UIZooming.BPC_PlayerState_UIZooming_C")
    (`Widget.SetVisibility` (`/Game/Core/Common/Helpers/BFL_Getters.GetCWMainStack`) "Collapsed")))

(event `/Game/Core/Common/Interfaces/BPI_ClickableObject.OnHoveredStart`
  (if (not (`self.IsCentered`))
    (set `self.IsAttached` false)
    (`self.PlayHoverTimeline`)))

(event `/Game/Core/Common/Interfaces/BPI_ClickableObject.OnHoveredEnd`
  (if (not (`self.IsCentered`))
    (`self.ReverseHoverTimeline`)))

(event `PlayHoverTimeline`
  (bind _output_get (set `self.PreviousPosition` (`self.K2_GetActorLocation`)))
  (set `self.Destination` (`KismetMathLibrary.MakeVector` (.x _output_get) (- (.y _output_get) 10.0) (.z _output_get)))
  (set `self.IsReversingHoverTimeline` false)
  (bind (_direction _alpha) (`Timeline|HoverTimeline` :!via `PlayFromStart` :!label _label)
    (:`Update`
      (`self.K2_SetActorLocation` (`KismetMathLibrary.VLerp` (`self.PreviousPosition`) (`self.Destination`) _alpha)))
    (:`Finished`
      (if (`self.IsReversingHoverTimeline`)
        (set `self.IsAttached` true)))))

(event `ReverseHoverTimeline`
  (set `self.IsReversingHoverTimeline` true)
  (goto _label :!via `Reverse`))

(event `PlayCenterTimeline`
  (bind (_cameralocation _camerarotation _cameraforwardvector) (`/Game/Core/Player/BP_BasePlayerController.GetCurrentCameraData` (`/Game/Core/Common/Helpers/BFL_Getters.GetMTGameController`)))
  (set `self.PreviousPosition` (`self.K2_GetActorLocation`))
  (bind _output_get (set `self.PreviousScale` (`self.GetActorScale3D`)))
  (set `self.DestinationScale` (* _output_get 2.2))
  (set `self.IsReversingCentered` false)
  (`KismetSystemLibrary.K2_ClearAndInvalidateTimerHandle` (`self.CombinationAngleFeedbackTimer`))
  (`SceneComponent.K2_SetRelativeRotation` (`self.SM_CombinationsNote`) (`self.InitialRotation`) false false)
  (bind (_direction _scalealpha _positionalpha) (`Timeline|CenterTimeline` :!via `PlayFromStart` :!label _label_2)
    (:`Update`
      (`self.K2_SetActorLocation` (`KismetMathLibrary.VLerp` (`self.PreviousPosition`) (+ _cameralocation (* _cameraforwardvector 200.0)) _positionalpha))
      (`self.SetActorScale3D` (`KismetMathLibrary.VLerp` (`self.PreviousScale`) (`self.DestinationScale`) _scalealpha)))
    (:`Finished`
      (if (`self.IsReversingCentered`)
        (set `self.IsCentered` false)
        (set `self.IsAttached` true)
        (`SceneComponent.K2_SetRelativeRotation` (`self.SM_CombinationsNote`) (`self.InitialRotation`) false true)
        (bind _returnvalue (`KismetSystemLibrary.K2_SetTimer` null "ProcessCombinationAngleFeedback" 0.25 true))
        (set `self.CombinationAngleFeedbackTimer` _returnvalue)))))

(event `ReverseCenterTimeline`
  (set `self.IsReversingCentered` true)
  (goto _label_2 :!via `ReverseFromEnd`))

(fn `OnCurrentCombinationsChanged`
  (params (CurrentCombination :type "/Game/Core/Player/E_Combinations Enum" :default "NewEnumerator6"))
  (switch `/Game/Core/Player/E_Combinations` CurrentCombination
    (:`NewEnumerator6`
      (`MeshComponent.SetOverlayMaterial` (`self.SM_CombinationsNote`) null)
      (set `self.ActiveCombination` false)
      (`KismetSystemLibrary.K2_ClearAndInvalidateTimerHandle` (`self.CombinationAngleFeedbackTimer`))
      (`SceneComponent.K2_SetRelativeRotation` (`self.SM_CombinationsNote`) (`self.InitialRotation`) false true))
    (:`NewEnumerator0`
      (if (`/Game/Core/Player/BP_BasePlayerController.InputsActive` (`/Game/Core/Common/Helpers/BFL_Getters.GetMTGameController`)) :!label _label
        (`MeshComponent.SetOverlayMaterial` (`self.SM_CombinationsNote`) "/Game/Materials/M_Outline_CombinationsNote.M_Outline_CombinationsNote")
        (bind _returnvalue (`KismetSystemLibrary.K2_SetTimer` null "ProcessCombinationAngleFeedback" 0.25 true))
        (set `self.CombinationAngleFeedbackTimer` _returnvalue)
        (else
          (`MeshComponent.SetOverlayMaterial` (`self.SM_CombinationsNote`) null)))
      (set `self.ActiveCombination` true))
    (:`NewEnumerator1`
      (goto _label))
    (:`NewEnumerator2`
      (goto _label))
    (:`NewEnumerator3`
      (goto _label))
    (:`NewEnumerator4`
      (goto _label))
    (:`NewEnumerator5`
      (goto _label))))

(fn `OnInputsActivationToggled`
  (params (AreInputsActive :type Boolean))
  (if AreInputsActive
    (`MaterialInstanceDynamic.SetScalarParameterValue` (`self.DMI_Note`) "EmissiveDiminisher" 1.0)
    (if (`self.ActiveCombination`)
      (`MeshComponent.SetOverlayMaterial` (`self.SM_CombinationsNote`) "/Game/Materials/M_Outline_CombinationsNote.M_Outline_CombinationsNote")
      (bind _returnvalue (`KismetSystemLibrary.K2_SetTimer` null "ProcessCombinationAngleFeedback" 0.25 true))
      (set `self.CombinationAngleFeedbackTimer` _returnvalue)
      (else
        (`MeshComponent.SetOverlayMaterial` (`self.SM_CombinationsNote`) null)
        (`KismetSystemLibrary.K2_ClearAndInvalidateTimerHandle` (`self.CombinationAngleFeedbackTimer`))
        (`SceneComponent.K2_SetRelativeRotation` (`self.SM_CombinationsNote`) (`self.InitialRotation`) false true)))
    (else
      (`MaterialInstanceDynamic.SetScalarParameterValue` (`self.DMI_Note`) "EmissiveDiminisher" 20.0)
      (`MeshComponent.SetOverlayMaterial` (`self.SM_CombinationsNote`) null))))

(fn `ProcessCombinationAngleFeedback`
  (bind (_initialrotation_roll _initialrotation_pitch _initialrotation_yaw) (`KismetMathLibrary.BreakRotator` (`self.InitialRotation`)))
  (`SceneComponent.K2_SetRelativeRotation` (`self.SM_CombinationsNote`) (`KismetMathLibrary.MakeRotator` (+ _initialrotation_roll (`KismetMathLibrary.RandomFloatInRange` -2.5 2.5)) _initialrotation_pitch _initialrotation_yaw) false false))

(fn `ProcessTiltBehavior`
  (bind (_returnvalue_x _returnvalue_y) (`KismetMathLibrary.BreakVector2D` (`WidgetLayoutLibrary.GetViewportSize`)))
  (bind (_locationx _locationy) (`PlayerController.GetMousePosition` (`/Game/Core/Common/Helpers/BFL_Getters.GetMTGameController`)))
  (`/Engine/EditorBlueprintResources/StandardMacros.IsValid` (`/Game/Core/Common/Helpers/BFL_Getters.GetMTGameController`)
    (:`Is Valid`
      (`SceneComponent.K2_SetRelativeRotation` (`self.SM_CombinationsNote`) (`KismetMathLibrary.RInterpTo` (`SceneComponent.RelativeRotation` (`self.SM_CombinationsNote`)) (`KismetMathLibrary.MakeRotator` (* (`KismetMathLibrary.MapRangeClamped` (/ _locationx _returnvalue_x) 0.0 1.0 -1.0 1.0) (`self.MaxTilt`) -1.0) (* (`KismetMathLibrary.MapRangeClamped` (/ _locationy _returnvalue_y) 0.0 1.0 -1.0 1.0) (`self.MaxTilt`) 1.0 1.0) 175.0) (`GameplayStatics.GetWorldDeltaSeconds`) 1.0) false false)
      (`SceneComponent.K2_SetRelativeRotation` (`self.Scene`) (`KismetMathLibrary.RInterpTo` (`SceneComponent.RelativeRotation` (`self.SM_CombinationsNote`)) (`KismetMathLibrary.MakeRotator` (* (`KismetMathLibrary.MapRangeClamped` (/ _locationx _returnvalue_x) 0.0 1.0 -1.0 1.0) (`self.MaxTilt`) -1.0) (* (`KismetMathLibrary.MapRangeClamped` (/ _locationy _returnvalue_y) 0.0 1.0 -1.0 1.0) (`self.MaxTilt`) 1.0 1.0) 175.0) (`GameplayStatics.GetWorldDeltaSeconds`) 1.0) false false))))

(fn `StopCenteringBehavior`
  (`self.ReverseCenterTimeline`)
  (`Widget.SetVisibility` (`/Game/Core/Common/Helpers/BFL_Getters.GetCWMainStack`) "Visible"))

(fn `UserConstructionScript`)