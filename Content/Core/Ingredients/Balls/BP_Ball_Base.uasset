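; BP_Ball_Base is a base ball actor that travels along an assigned spline and visually reflects its accumulated score.
; Tick advances it at constant speed, scaled by the game instance's PauseTick.
; AddScore maps CurrentScore to a feedback alpha across two consecutive threshold ranges.
; Tick uses that alpha to lerp a dynamic material's opacity, color, roughness and emissive, shifting from grey through translucent white to glowing pink.
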(event `self.ReceiveBeginPlay`
  (bind _returnvalue (`KismetMaterialLibrary.CreateDynamicMaterialInstance` "/Game/Assets/3D/Environment/Materials/M_Ball.M_Ball"))
  (bind _output_get (set `self.DMI_Ball` _returnvalue))
  (`PrimitiveComponent.SetMaterial` (`self.SM_Ball`) 0 _output_get))

(event `self.ReceiveTick`
  (params (DeltaSeconds :type "Float (single-precision)"))
  (`|ExecutionSequence`
    (:`then_0`
      (bind _output_get (set `self.DistanceAlongSpline` (+ (`self.DistanceAlongSpline`) (* 50.0 (`GameplayStatics.GetWorldDeltaSeconds`) (`/Game/Core/Game/BP_GameInstance.PauseTick` (`/Game/Core/Common/Helpers/BFL_Getters.GetMTGameInstance`))))))
      (`self.K2_SetActorLocation` (`SplineComponent.GetLocationAtDistanceAlongSpline` (`self.AssignedSpline`) _output_get "World")))
    (:`then_1`
      (if (not (`self.IsOnSecondLerp`))
        (`MaterialInstanceDynamic.SetScalarParameterValue` (`self.DMI_Ball`) "Opacity" (`KismetMathLibrary.Lerp` 1.0 0.5 (`self.FeedbackAlpha`)))
        (`MaterialInstanceDynamic.SetVectorParameterValue` (`self.DMI_Ball`) "BallColor" (`KismetMathLibrary.LinearColorLerp` (struct :`R` 0.296138 :`G` 0.296138 :`B` 0.296138 :`A` 1.0) (struct :`R` 1.0 :`G` 1.0 :`B` 1.0 :`A` 1.0) (`self.FeedbackAlpha`)))
        (`MaterialInstanceDynamic.SetScalarParameterValue` (`self.DMI_Ball`) "Roughness" (`KismetMathLibrary.Lerp` 0.5 1.0 (`self.FeedbackAlpha`)))
        (`MaterialInstanceDynamic.SetScalarParameterValue` (`self.DMI_Ball`) "EmissiveStrength" (`KismetMathLibrary.Lerp` 0.0 0.0 (`self.FeedbackAlpha`)))
        (else
          (`MaterialInstanceDynamic.SetScalarParameterValue` (`self.DMI_Ball`) "Opacity" (`KismetMathLibrary.Lerp` 0.5 1.0 (`self.FeedbackAlpha`)))
          (`MaterialInstanceDynamic.SetVectorParameterValue` (`self.DMI_Ball`) "BallColor" (`KismetMathLibrary.LinearColorLerp` (struct :`R` 1.0 :`G` 1.0 :`B` 1.0 :`A` 1.0) (struct :`R` 1.0 :`G` 0.25883 :`B` 0.924878 :`A` 1.0) (`self.FeedbackAlpha`)))
          (`MaterialInstanceDynamic.SetScalarParameterValue` (`self.DMI_Ball`) "Roughness" (`KismetMathLibrary.Lerp` 1.0 0.7 (`self.FeedbackAlpha`)))
          (`MaterialInstanceDynamic.SetScalarParameterValue` (`self.DMI_Ball`) "EmissiveStrength" (`KismetMathLibrary.Lerp` 0.0 0.2 (`self.FeedbackAlpha`))))))))

(fn `AddScore`
  (params (AddedScore :type "Float (double-precision)"))
  (set `self.CurrentScore` (+ (`self.CurrentScore`) AddedScore))
  (if (and (>= (`self.CurrentScore`) (`self.FirstLerpMaximum`)) (not (`self.IsOnSecondLerp`)))
    (set `self.IsOnSecondLerp` true))
  (if (not (`self.IsOnSecondLerp`))
    (set `self.FeedbackAlpha` (`KismetMathLibrary.MapRangeClamped` (`self.CurrentScore`) 0.0 (`self.FirstLerpMaximum`) 0.0 1.0))
    (else
      (set `self.FeedbackAlpha` (`KismetMathLibrary.MapRangeClamped` (`self.CurrentScore`) (`self.FirstLerpMaximum`) (`self.SecondLerpMaximum`) 0.0 1.0)))))

(fn `UserConstructionScript`)