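; Base monster actor that idles in place and spawns each round's wave of balls.
; A looping timer picks random height offsets for a timeline bob, while Tick eases the pivot sideways toward the player during the Idle game state and back to base otherwise.
; SpawnWave uses a delayed-loop macro to spawn the round's balls on tag-matched splines and register them with the game state.
; The Niagara spline visual is left unconnected.
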(event `self.ReceiveBeginPlay`
  (set `self.BasePosition` (`SceneComponent.K2_GetComponentLocation` (`self.CenteredPivot`)))
  (`KismetSystemLibrary.K2_SetTimer` null "ChangeIdleZDestination" 4.0 true)
  (`PrimitiveComponent.SetMaterial` (`self.SM_MonsterEyes`) 0 (`self.EyesMaterial`)))

(event `self.ReceiveTick`
  (params (DeltaSeconds :type "Float (single-precision)"))
  (bind (_returnvalue_x _returnvalue_y _returnvalue_z) (`KismetMathLibrary.BreakVector` (`SceneComponent.K2_GetComponentLocation` (`self.CenteredPivot`))))
  (bind (_returnvalue_x_2 _returnvalue_y_2) (`KismetMathLibrary.BreakVector` (`SceneComponent.K2_GetComponentLocation` (`self.CenteredPivot`))))
  (`|ExecutionSequence`
    (:`then_0`
      (`self.CalculateIdleYDestination`)
      (`SceneComponent.K2_SetWorldLocation` (`self.CenteredPivot`) (`KismetMathLibrary.MakeVector` _returnvalue_x (`KismetMathLibrary.FInterpTo` _returnvalue_y_2 (`self.IdleYDestination`) (`GameplayStatics.GetWorldDeltaSeconds`) (`self.YOffsetSpeed`)) _returnvalue_z) false false))))

(event `SpawnWave`
  (params (CurrentRound :type Integer))
  (bind _balls (break `/Game/Core/Common/Structs/S_RoundData` (`|GetArrayItem` (`self.Rounds`) (- CurrentRound 1))))
  (bind _index (`self.ForLoopWithDelay` 0 (- (`KismetArrayLibrary.Array_Length` _balls) 1) 1.0)
    (:`LoopBody`
      (bind (_ballclass _splinename) (break `/Game/Core/Common/Structs/S_BallConfig` (`|GetArrayItem` _balls _index)))
      (bind _returnvalue (`self.FindComponentByTag` "/Script/Engine.SplineComponent" _splinename))
      (bind _returnvalue_2 (`|SpawnActorFromClass` _ballclass (`KismetMathLibrary.MakeTransform` (`SplineComponent.GetLocationAtSplinePoint` _returnvalue 0 "World")) "Undefined" "MultiplyWithRoot" null _returnvalue null))
      (`/Game/Core/Game/BP_GameState.AddSpawnedBall` (`/Game/Core/Common/Helpers/BFL_Getters.GetMTGameState`) _returnvalue_2))))

(event `TriggerIdleMovement`
  (bind (_returnvalue_x _returnvalue_y _returnvalue_z) (`KismetMathLibrary.BreakVector` (`SceneComponent.K2_GetComponentLocation` (`self.CenteredPivot`))))
  (bind (_returnvalue_x_2 _returnvalue_y_2) (`KismetMathLibrary.BreakVector` (`SceneComponent.K2_GetComponentLocation` (`self.CenteredPivot`))))
  (set `self.PreviousZPosition` _returnvalue_z)
  (bind (_direction _lerpalpha) (`Timeline|IdleMovementTimeline` :!via `PlayFromStart`)
    (:`Update`
      (`SceneComponent.K2_SetWorldLocation` (`self.CenteredPivot`) (`KismetMathLibrary.MakeVector` _returnvalue_x_2 _returnvalue_y_2 (`KismetMathLibrary.Lerp` (`self.PreviousZPosition`) (`self.IdleZDestination`) _lerpalpha)) false false))))

(fn `CalculateIdleYDestination`
  (bind (_baseposition_x _baseposition_y) (`KismetMathLibrary.BreakVector` (`self.BasePosition`)))
  (bind (_baseposition_x_2 _baseposition_y_2) (`KismetMathLibrary.BreakVector` (`self.BasePosition`)))
  (`/Engine/EditorBlueprintResources/StandardMacros.IsValid` (`/Game/Core/Common/Helpers/BFL_Getters.GetMTPlayerCharacter`)
    (:`Is Valid`
      (if (== (`/Game/Core/Game/BP_GameState.CurrentState` (`/Game/Core/Common/Helpers/BFL_Getters.GetMTGameState`)) "/Game/Core/Game/States/BPC_GameState_Idle.BPC_GameState_Idle_C")
        (bind _output_get (set `self.IdleYOffset` (* (/ (- (.y (`self.K2_GetActorLocation` (`/Game/Core/Common/Helpers/BFL_Getters.GetMTPlayerCharacter`))) (.y (`SceneComponent.K2_GetComponentLocation` (`self.CenteredPivot`)))) 300.0) 25.0)))
        (set `self.IdleYDestination` (+ _output_get _baseposition_y_2))
        (set `self.YOffsetSpeed` 0.6)
        (else
          (bind _output_get_2 (set `self.IdleYOffset` 0.0))
          (set `self.IdleYDestination` (+ _output_get_2 _baseposition_y))
          (set `self.YOffsetSpeed` 2.0))))))

(fn `ChangeIdleZDestination`
  (bind (_baseposition_x _baseposition_y _baseposition_z) (`KismetMathLibrary.BreakVector` (`self.BasePosition`)))
  (bind _output_get (set `self.IdleZOffset` (`KismetMathLibrary.RandomFloatInRange` -10.0 10.0)))
  (set `self.IdleZDestination` (+ _output_get _baseposition_z))
  (`self.TriggerIdleMovement`))

(fn `UserConstructionScript`)