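; Dice component that performs the amplify effect on its AmplifiedDice, showing an area VFX while that dice's collision expands.
; On BeginPlay it binds to the dice's extend-finished event, resets its AOE collision data, spawns a Niagara system just below the mesh scaled to the amplification size, then starts the collision extension.
; When the extension finishes, the component destroys itself, and EndPlay removes the VFX.
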(event `self.ReceiveBeginPlay`
  (`self.DoBindings`)
  (`/Game/Core/Ingredients/Dices/BP_Dice.ResetDiceAOECollisionData` (`self.AmplifiedDice`))
  (`self.SpawnAmplificationVFX`)
  (`/Game/Core/Ingredients/Dices/BP_Dice.ExtendCollision` (`self.AmplifiedDice`) (`/Game/Core/Ingredients/Dices/BP_Dice.AmplificationAOESize` (`self.AmplifiedDice`))))

(event `self.ReceiveEndPlay`
  (params (EndPlayReason :type "EEndPlayReason Enum" :default "Destroyed"))
  (`self.DestroyAmplificationVFX`))

(event `DoBindings`
  (add `/Game/Core/Ingredients/Dices/BP_Dice.OnCollisionExtendFinished` (`self.AmplifiedDice`) (`|CreateDelegate` :!event `OnCollisionExtendFinished`)))

(fn `DestroyAmplificationVFX`
  (bind _ns_diceamplification (`self.NS_DiceAmplification`))
  (`/Engine/EditorBlueprintResources/StandardMacros.IsValid` _ns_diceamplification
    (:`Is Valid`
      (`self.K2_DestroyComponent` _ns_diceamplification))))

(fn `OnCollisionExtendFinished`
  (`self.K2_DestroyComponent`))

(fn `SpawnAmplificationVFX`
  (bind (_returnvalue_x _returnvalue_y _returnvalue_z) (`KismetMathLibrary.BreakVector` (`SceneComponent.K2_GetComponentLocation` (`/Game/Core/Ingredients/Dices/BP_Dice.SM_Dice` (`self.AmplifiedDice`)))))
  (bind _returnvalue (`NiagaraFunctionLibrary.SpawnSystemAtLocation` "/Game/VFX/Dices/NS_Dice_Amplification.NS_Dice_Amplification" (`KismetMathLibrary.MakeVector` _returnvalue_x _returnvalue_y (- _returnvalue_z 3.0))))
  (set `self.NS_DiceAmplification` _returnvalue)
  (`NiagaraComponent.SetVariableFloat` (`self.NS_DiceAmplification`) "MaxScale" (`/Game/Core/Ingredients/Dices/BP_Dice.AmplificationAOESize` (`self.AmplifiedDice`)))
  (`self.Activate` (`self.NS_DiceAmplification`) true))