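; Dice component that starts an attraction area effect on its AttractingDice, with matching Niagara VFX.
; On BeginPlay it resets the dice's AOE collision data, spawns the effect just below the dice mesh, and extends collision to AttractionAOESize.
; The same size drives the effect's MaxScale, and EndPlay destroys the effect.
; It binds to the dice's collision-extend-finished event, and its OnCollisionExtendFinished function is empty.
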(event `self.ReceiveBeginPlay`
  (`self.DoBindings`)
  (`/Game/Core/Ingredients/Dices/BP_Dice.ResetDiceAOECollisionData` (`self.AttractingDice`))
  (`self.SpawnAttractingVFX`)
  (`/Game/Core/Ingredients/Dices/BP_Dice.ExtendCollision` (`self.AttractingDice`) (`/Game/Core/Ingredients/Dices/BP_Dice.AttractionAOESize` (`self.AttractingDice`))))

(event `self.ReceiveEndPlay`
  (params (EndPlayReason :type "EEndPlayReason Enum" :default "Destroyed"))
  (`self.DestroyAttractingVFX`))

(event `DoBindings`
  (add `/Game/Core/Ingredients/Dices/BP_Dice.OnCollisionExtendFinished` (`self.AttractingDice`) (`|CreateDelegate` :!event `OnCollisionExtendFinished`)))

(fn `DestroyAttractingVFX`
  (bind _ns_diceattraction (`self.NS_DiceAttraction`))
  (`/Engine/EditorBlueprintResources/StandardMacros.IsValid` _ns_diceattraction
    (:`Is Valid`
      (`self.K2_DestroyComponent` _ns_diceattraction))))

(fn `OnCollisionExtendFinished`)

(fn `SpawnAttractingVFX`
  (bind (_returnvalue_x _returnvalue_y _returnvalue_z) (`KismetMathLibrary.BreakVector` (`SceneComponent.K2_GetComponentLocation` (`/Game/Core/Ingredients/Dices/BP_Dice.SM_Dice` (`self.AttractingDice`)))))
  (bind _returnvalue (`NiagaraFunctionLibrary.SpawnSystemAtLocation` "/Game/VFX/Dices/NS_Dice_Attraction.NS_Dice_Attraction" (`KismetMathLibrary.MakeVector` _returnvalue_x _returnvalue_y (- _returnvalue_z 3.0))))
  (set `self.NS_DiceAttraction` _returnvalue)
  (`NiagaraComponent.SetVariableFloat` (`self.NS_DiceAttraction`) "MaxScale" (`/Game/Core/Ingredients/Dices/BP_Dice.AttractionAOESize` (`self.AttractingDice`)))
  (`self.Activate` (`self.NS_DiceAttraction`) true))