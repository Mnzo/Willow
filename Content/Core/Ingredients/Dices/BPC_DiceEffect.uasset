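; Actor component on a BP_Dice that periodically adds score to an affected ball.
; On BeginPlay it caches the owning die, triggers once immediately and starts a looping timer at TickTime.
; Each trigger scales the die's face value into score, also applying the player character's MultiplierMap entry for that value when the die is in a combination.
; It then spawns a Niagara hit effect at the die, setting its beam end to the ball's location before activation.
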(event `self.ReceiveBeginPlay`
  (`KismetSystemLibrary.K2_SetTimer` null "TriggerEffect" (`self.TickTime`) true)
  (set `self.DiceAffecting` (cast `/Game/Core/Ingredients/Dices/BP_Dice` (`self.GetOwner`) :!pure true))
  (`self.TriggerEffect`))

(fn `TriggerEffect`
  (if (not (`/Game/Core/Ingredients/Dices/BP_Dice.IsDiceInCombination` (`self.DiceAffecting`)))
    (`/Game/Core/Ingredients/Balls/BP_Ball_Base.AddScore` (`self.AffectedBall`) (* (`KismetMathLibrary.Conv_IntToDouble` (`/Game/Core/Ingredients/Dices/BP_Dice.GetFaceRealValue` (`self.DiceAffecting`))) 10.0))
    (else
      (`/Game/Core/Ingredients/Balls/BP_Ball_Base.AddScore` (`self.AffectedBall`) (* (`KismetMathLibrary.Conv_IntToDouble` (* (`/Game/Core/Ingredients/Dices/BP_Dice.GetFaceRealValue` (`self.DiceAffecting`)) (`BlueprintMapLibrary.Map_Find` (`/Game/Core/Player/BP_PlayerCharacter.MultiplierMap` (`/Game/Core/Common/Helpers/BFL_Getters.GetMTPlayerCharacter`)) (`/Game/Core/Ingredients/Dices/BP_Dice.GetFaceRealValue` (`self.DiceAffecting`))))) 10.0))))
  (bind _returnvalue (`NiagaraFunctionLibrary.SpawnSystemAtLocation` "/Game/VFX/Dices/NS_Dice_Hit.NS_Dice_Hit" (`SceneComponent.K2_GetComponentLocation` (`/Game/Core/Ingredients/Dices/BP_Dice.SM_Dice` (`self.DiceAffecting`))) (struct) (1.0 1.0 1.0) true false))
  (`NiagaraComponent.SetVariablePosition` _returnvalue "BeamEndPosition" (`Actor.K2_GetActorLocation` (`self.AffectedBall`)))
  (`self.Activate` _returnvalue true))