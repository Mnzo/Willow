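; Physics-driven die that the player rotates or selects, throws onto the game board, and uses as an area effect on balls.
; Once at rest during throwing, an upward-face trace finds its BP_Face value, which feeds a value widget and the player's combination logic.
; On activation, that value sizes the AOE sphere and Niagara effect.
; Overlapping balls get per-ball BPC_DiceEffect components, whose tick time uses fire rate for dice in combinations.
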(event `self.ReceiveBeginPlay`
  (`PrimitiveComponent.SetMaterial` (`self.SM_Dice`) 0 (`self.DiceMaterial`))
  (`self.ProcessSpawn`)
  (`self.InitializeFaces`)
  (add `/Game/Core/Player/BP_PlayerCharacter.OnCurrentCombinationChanged` (`/Game/Core/Common/Helpers/BFL_Getters.GetMTPlayerCharacter`) (`|CreateDelegate` :!event `OnCurrentCombinationChanged`)))

(event `/Game/Core/Common/Interfaces/BPI_ClickableObject.OnClickStart`
  (`/Engine/EditorBlueprintResources/StandardMacros.IsValid` (`/Game/Core/Player/BP_PlayerCharacter.CurrentStateObject` (`/Game/Core/Common/Helpers/BFL_Getters.GetMTPlayerCharacter`))
    (:`Is Valid`
      (if (and (`/Game/Core/Player/States/BPC_PlayerState_Base.CanRotateDices` (`/Game/Core/Player/BP_PlayerCharacter.CurrentStateObject` (`/Game/Core/Common/Helpers/BFL_Getters.GetMTPlayerCharacter`))) (not (`self.IsStopped`)))
        (`self.StopRotation`)
        (set `self.WantedRotation` (`KismetMathLibrary.Conv_RotatorToQuaternion` (`SceneComponent.K2_GetComponentRotation` (`self.SM_Dice`))))
        (elif (`/Game/Core/Player/States/BPC_PlayerState_Base.CanSelectDices` (`/Game/Core/Player/BP_PlayerCharacter.CurrentStateObject` (`/Game/Core/Common/Helpers/BFL_Getters.GetMTPlayerCharacter`)))
          (`/Game/Core/Player/BP_PlayerCharacter.SelectDice` (`/Game/Core/Common/Helpers/BFL_Getters.GetMTPlayerCharacter`) self))))))

(event `/Game/Core/Common/Interfaces/BPI_ClickableObject.OnClickUpdate`
  (`/Engine/EditorBlueprintResources/StandardMacros.IsValid` (`/Game/Core/Player/BP_PlayerCharacter.CurrentStateObject` (`/Game/Core/Common/Helpers/BFL_Getters.GetMTPlayerCharacter`))
    (:`Is Valid`
      (if (and (`/Game/Core/Player/States/BPC_PlayerState_Base.CanRotateDices` (`/Game/Core/Player/BP_PlayerCharacter.CurrentStateObject` (`/Game/Core/Common/Helpers/BFL_Getters.GetMTPlayerCharacter`))) (not (`self.IsStopped`)))
        (bind _output_get (set `self.WantedRotation` (`self.CalculateWantedRotation`)))
        (`SceneComponent.K2_SetWorldRotation` (`self.SM_Dice`) (`KismetMathLibrary.Quat_Rotator` _output_get) false false)))))

(event `/Game/Core/Common/Interfaces/BPI_ClickableObject.OnClickStop`
  (`/Engine/EditorBlueprintResources/StandardMacros.IsValid` (`/Game/Core/Player/BP_PlayerCharacter.CurrentStateObject` (`/Game/Core/Common/Helpers/BFL_Getters.GetMTPlayerCharacter`))
    (:`Is Valid`
      (if (and (`/Game/Core/Player/States/BPC_PlayerState_Base.CanRotateDices` (`/Game/Core/Player/BP_PlayerCharacter.CurrentStateObject` (`/Game/Core/Common/Helpers/BFL_Getters.GetMTPlayerCharacter`))) (not (`self.IsStopped`)))
        (`self.ResetRotation`)))))

(event `self.SM_Dice.OnComponentHit`
  (params (HitComponent :type "PrimitiveComponent Object Reference") (OtherActor :type "Actor Object Reference") (OtherComp :type "PrimitiveComponent Object Reference") (NormalImpulse :type "Vector Structure") (Hit :type "HitResult Structure (by ref)"))
  (bind _sm_dice (`self.SM_Dice`))
  (cast `/Game/Core/Ingredients/BP_GameBoard` OtherActor
    (:`then`
      (if (== (`PrimitiveComponent.GetLinearDamping` (`self.SM_Dice`)) 0.0)
        (`PrimitiveComponent.SetAngularDamping` _sm_dice 1.8)
        (`PrimitiveComponent.SetLinearDamping` _sm_dice 1.8)))
    (:`CastFailed`
      (bind _asbp_dice (cast `/Game/Core/Ingredients/Dices/BP_Dice` OtherActor))
      (if (and (`self.IsStopped`) (`self.IsPreValidated`))
        (set `self.IsStopped` false)
        (`PrimitiveComponent.AddImpulse` (`self.SM_Dice`) (* (`KismetMathLibrary.Normal` (- (`self.K2_GetActorLocation` _asbp_dice) (`self.K2_GetActorLocation`))) 200.0) "None" false)
        (set `self.CurrentFaceValue` 0)
        (`/Game/Core/Player/BP_PlayerCharacter.RemoveCombination` (`/Game/Core/Common/Helpers/BFL_Getters.GetMTPlayerCharacter`))))))

(event `self.ReceiveTick`
  (params (DeltaSeconds :type "Float (single-precision)"))
  (bind _sm_dice (`self.SM_Dice`))
  (`|ExecutionSequence`
    (:`then_0`
      (if (== (`/Game/Core/Game/BP_GameState.CurrentState` (`/Game/Core/Common/Helpers/BFL_Getters.GetMTGameState`)) "/Game/Core/Game/States/BPC_GameState_GB_Throwing.BPC_GameState_GB_Throwing_C")
        (bind _returnvalue (`PrimitiveComponent.GetPhysicsLinearVelocity` _sm_dice "None"))
        (if (and (< (`KismetMathLibrary.VSize` _returnvalue) 8.0) (< (`KismetMathLibrary.VSize` (`PrimitiveComponent.GetPhysicsAngularVelocityInDegrees` _sm_dice "None")) 5.0) (not (`self.IsStopped`)))
          (`self.StopDice`)
          (if (`/Game/Core/Player/BP_PlayerCharacter.AreDicesStopped` (`/Game/Core/Common/Helpers/BFL_Getters.GetMTPlayerCharacter`))
            (`/Game/Core/Player/BP_PlayerCharacter.ProcessDicesAllStopped` (`/Game/Core/Common/Helpers/BFL_Getters.GetMTPlayerCharacter`))))))))

(event `/Game/Core/Common/Interfaces/BPI_ClickableObject.OnHoveredStart`
  (`/Engine/EditorBlueprintResources/StandardMacros.IsValid` (`/Game/Core/Game/BP_GameState.CurrentStateObject` (`/Game/Core/Common/Helpers/BFL_Getters.GetMTGameState`))
    (:`Is Valid`
      (set `self.IsHovered` true)
      (if (== (`/Game/Core/Game/BP_GameState.CurrentState` (`/Game/Core/Common/Helpers/BFL_Getters.GetMTGameState`)) "/Game/Core/Game/States/BPC_GameState_GB_Evaluating.BPC_GameState_GB_Evaluating_C")
        (`WidgetComponent.SetTintColorAndOpacity` (`self.W_DiceValue`) (struct :`R` 1.0 :`G` 1.0 :`B` 1.0 :`A` 1.0))))))

(event `/Game/Core/Common/Interfaces/BPI_ClickableObject.OnHoveredEnd`
  (`/Engine/EditorBlueprintResources/StandardMacros.IsValid` (`/Game/Core/Game/BP_GameState.CurrentStateObject` (`/Game/Core/Common/Helpers/BFL_Getters.GetMTGameState`))
    (:`Is Valid`
      (set `self.IsHovered` false)
      (if (== (`/Game/Core/Game/BP_GameState.CurrentState` (`/Game/Core/Common/Helpers/BFL_Getters.GetMTGameState`)) "/Game/Core/Game/States/BPC_GameState_GB_Evaluating.BPC_GameState_GB_Evaluating_C")
        (`WidgetComponent.SetTintColorAndOpacity` :`self` (`self.W_DiceValue`))))))

(event `self.DiceAOECollision.OnComponentBeginOverlap`
  (params (OverlappedComponent :type "PrimitiveComponent Object Reference") (OtherActor :type "Actor Object Reference") (OtherComp :type "PrimitiveComponent Object Reference") (OtherBodyIndex :type Integer) (bFromSweep :type Boolean) (SweepResult :type "HitResult Structure (by ref)"))
  (bind _asbp_ball_base (cast `/Game/Core/Ingredients/Balls/BP_Ball_Base` OtherActor))
  (set `self.NewlyAffectedBall` _asbp_ball_base)
  (if (`self.IsDiceInCombination`)
    (set `self.EffectTickTime` (/ 0.2 (/ (`BlueprintMapLibrary.Map_Find` (`/Game/Core/Player/BP_PlayerCharacter.FireRateMap` (`/Game/Core/Common/Helpers/BFL_Getters.GetMTPlayerCharacter`)) (`self.GetFaceRealValue`)) 100.0)))
    (else
      (set `self.EffectTickTime` 0.2)))
  (bind _returnvalue (`|AddComponentByClass` "/Game/Core/Ingredients/Dices/BPC_DiceEffect.BPC_DiceEffect_C" (`self.NewlyAffectedBall`) (`self.EffectTickTime`)))
  (`BlueprintMapLibrary.Map_Add` (`self.DiceEffectsPerBall`) (`self.NewlyAffectedBall`) _returnvalue))

(event `self.DiceAOECollision.OnComponentEndOverlap`
  (params (OverlappedComponent :type "PrimitiveComponent Object Reference") (OtherActor :type "Actor Object Reference") (OtherComp :type "PrimitiveComponent Object Reference") (OtherBodyIndex :type Integer))
  (bind _asbp_ball_base (cast `/Game/Core/Ingredients/Balls/BP_Ball_Base` OtherActor))
  (`ActorComponent.K2_DestroyComponent` (`BlueprintMapLibrary.Map_Find` (`self.DiceEffectsPerBall`) _asbp_ball_base))
  (`BlueprintMapLibrary.Map_Remove` (`self.DiceEffectsPerBall`) _asbp_ball_base))

(event `self.ReceiveDestroyed`
  (bind _dicedecal (`self.DiceDecal`))
  (bind _ns_diceaoe (`self.NS_DiceAOE`))
  (`/Engine/EditorBlueprintResources/StandardMacros.IsValid` _ns_diceaoe
    (:`Is Valid`
      (`ActorComponent.K2_DestroyComponent` _ns_diceaoe))
    (:`Is Not Valid`
      _))
  (`/Engine/EditorBlueprintResources/StandardMacros.IsValid` _dicedecal
    (:`Is Valid`
      (`ActorComponent.K2_DestroyComponent` _dicedecal))))

(event `ResetRotation`
  (bind (_direction _rotationdelta) (`Timeline|DiceRotationTimeline` :!via `PlayFromStart` :!label _label)
    (:`Update`
      (`SceneComponent.K2_SetWorldRotation` (`self.SM_Dice`) (`KismetMathLibrary.Quat_Rotator` (`KismetMathLibrary.Quat_Slerp` (`KismetMathLibrary.Conv_RotatorToQuaternion` (`SceneComponent.K2_GetComponentRotation` (`self.SM_Dice`))) (`self.InitialRotation`) _rotationdelta)) false false))))

(event `StopRotation`
  (goto _label :!via `Stop`))

(fn `ActivatePostThrowCollision`
  (`PrimitiveComponent.SetCollisionProfileName` (`self.SM_Dice`) "DicePostThrow" true))

(fn `AdjustSpawnTransformAndRetry`
  (locals (NewPosition :type "Vector Structure"))
  (bind _dicesspawnzone (`/Game/Core/Player/Cameras/BP_PlayerCamera_PreThrow.DicesSpawnZone` (cast `/Game/Core/Player/Cameras/BP_PlayerCamera_PreThrow` (`/Game/Core/Game/BP_GameInstance.GetCameraPreThrow` (`/Game/Core/Common/Helpers/BFL_Getters.GetMTGameInstance`)) :!pure true)))
  (set `local.NewPosition` (`KismetMathLibrary.RandomPointInBoundingBox` (`SceneComponent.K2_GetComponentLocation` _dicesspawnzone) (`BoxComponent.BoxExtent` _dicesspawnzone)))
  (`SceneComponent.K2_SetWorldLocation` (`self.SM_Dice`) (`local.NewPosition`) false true)
  (`SceneComponent.K2_SetWorldRotation` (`self.SM_Dice`) (`KismetMathLibrary.RandomRotator` false) false true))

(fn `CalculateWantedRotation`
  (returns (WantedRotation :type "Quat Structure"))
  (bind _mtgamecontroller (`/Game/Core/Common/Helpers/BFL_Getters.GetMTGameController`))
  (bind _playercameramanager (`PlayerController.PlayerCameraManager` (`/Game/Core/Common/Helpers/BFL_Getters.GetMTGameController`)))
  (bind _returnvalue (- (`/Game/Core/Player/BP_BasePlayerController.GetCurrentMousePosition` _mtgamecontroller) (`/Game/Core/Player/BP_PlayerController_Game.FirstClick2DPosition` _mtgamecontroller)))
  (bind (_returnvalue_x _returnvalue_y) (`KismetMathLibrary.BreakVector2D` (`KismetMathLibrary.Normal2D` (* _returnvalue (-1.0 -1.0)))))
  (return (`KismetMathLibrary.Quat_Normalized` (* (`KismetMathLibrary.Conv_RotatorToQuaternion` (`KismetMathLibrary.RotatorFromAxisAndAngle` (+ (* _returnvalue_x (`self.GetActorUpVector` _playercameramanager)) (* _returnvalue_y (`self.GetActorRightVector` _playercameramanager))) (`KismetSystemLibrary.MakeLiteralDouble` (`KismetMathLibrary.DegreesToRadians` (* (`self.RotationSpeed`) (`KismetMathLibrary.VSize2D` _returnvalue) (`GameplayStatics.GetWorldDeltaSeconds`)))))) (`self.WantedRotation`)))))

(fn `EnterActivationPhase`
  (`self.SpawnDiceVFX`)
  (`self.UpdateDiceCollision`))

(fn `EnterEvaluatingPhase`
  (`self.ForcePreHoveredAction`))

(fn `FindFaceValue`
  (bind _sm_dice (`self.SM_Dice`))
  (bind (_returnvalue_x _returnvalue_y _returnvalue_z) (`KismetMathLibrary.BreakVector` (`SceneComponent.K2_GetComponentLocation` _sm_dice)))
  (bind _outhit (`KismetSystemLibrary.LineTraceSingle` (`KismetMathLibrary.MakeVector` _returnvalue_x _returnvalue_y (+ _returnvalue_z 100.0)) (`SceneComponent.K2_GetComponentLocation` _sm_dice) "TraceTypeQuery2"))
  (bind _asbp_face (cast `/Game/Core/Ingredients/Dices/BP_Face` (`.HitActor` (`GameplayStatics.BreakHitResult` _outhit))))
  (set `self.CurrentFaceValue` (select `/Game/Core/Ingredients/Dices/E_FaceTypes` (`/Game/Core/Ingredients/Dices/BP_Face.FaceType` _asbp_face) :`NewEnumerator0` 1 :`NewEnumerator1` 2 :`NewEnumerator2` 3 :`NewEnumerator3` 4 :`NewEnumerator4` 5 :`NewEnumerator5` 6 :`NewEnumerator6` 111 :`NewEnumerator7` 211 :`NewEnumerator8` 311 :`NewEnumerator9` 411 :`NewEnumerator10` 511)))

(fn `ForcePreHoveredAction`
  (if (`self.IsHovered`)
    (`self.OnHoveredStart`)))

(fn `GetFaceRealValue`
  (returns (FaceRealValue :type Integer))
  (bind _currentfacevalue (`self.CurrentFaceValue`))
  (if (== _currentfacevalue 1)
    (return 1)
    (elif (== _currentfacevalue 2)
      (return 2)
      (elif (== _currentfacevalue 3)
        (return 3)
        (elif (== _currentfacevalue 4)
          (return 4)
          (elif (== _currentfacevalue 5)
            (return 5)
            (elif (== _currentfacevalue 6)
              (return 6)
              (elif (== _currentfacevalue 111)
                (return 1)
                (elif (== _currentfacevalue 211)
                  (return 2)
                  (elif (== _currentfacevalue 311)
                    (return 3)
                    (elif (== _currentfacevalue 411)
                      (return 4)
                      (elif (== _currentfacevalue 511)
                        (return 5)
                        (else
                          (return -1))))))))))))))

(fn `InitializeFaces`
  (bind _asbp_face (cast `/Game/Core/Ingredients/Dices/BP_Face` (`ChildActorComponent.ChildActor` (`self.FaceTop`))))
  (set `/Game/Core/Ingredients/Dices/BP_Face.FaceType` (`self.DefaultFaceTop`) _asbp_face)
  (bind _asbp_face_2 (cast `/Game/Core/Ingredients/Dices/BP_Face` (`ChildActorComponent.ChildActor` (`self.FaceBottom`))))
  (set `/Game/Core/Ingredients/Dices/BP_Face.FaceType` (`self.DefaultFaceBottom`) _asbp_face_2)
  (bind _asbp_face_3 (cast `/Game/Core/Ingredients/Dices/BP_Face` (`ChildActorComponent.ChildActor` (`self.FaceBack`))))
  (set `/Game/Core/Ingredients/Dices/BP_Face.FaceType` (`self.DefaultFaceBack`) _asbp_face_3)
  (bind _asbp_face_4 (cast `/Game/Core/Ingredients/Dices/BP_Face` (`ChildActorComponent.ChildActor` (`self.FaceFront`))))
  (set `/Game/Core/Ingredients/Dices/BP_Face.FaceType` (`self.DefaultFaceFront`) _asbp_face_4)
  (bind _asbp_face_5 (cast `/Game/Core/Ingredients/Dices/BP_Face` (`ChildActorComponent.ChildActor` (`self.FaceRight`))))
  (set `/Game/Core/Ingredients/Dices/BP_Face.FaceType` (`self.DefaultFaceRight`) _asbp_face_5)
  (bind _asbp_face_6 (cast `/Game/Core/Ingredients/Dices/BP_Face` (`ChildActorComponent.ChildActor` (`self.FaceLeft`))))
  (set `/Game/Core/Ingredients/Dices/BP_Face.FaceType` (`self.DefaultFaceLeft`) _asbp_face_6))

(fn `IsDiceInCombination`
  (returns (IsInCombination :type Boolean))
  (bind _mtplayercharacter (`/Game/Core/Common/Helpers/BFL_Getters.GetMTPlayerCharacter`))
  (`/Engine/EditorBlueprintResources/StandardMacros.IsValid` _mtplayercharacter
    (:`Is Valid`
      (return (!= (`KismetArrayLibrary.Array_Find` (`/Game/Core/Player/BP_PlayerCharacter.DicesInCombination` _mtplayercharacter) self) -1)))))

(fn `IsPersonaFace`
  (returns (IsPersona :type Boolean))
  (bind _currentfacevalue (`self.CurrentFaceValue`))
  (if (== _currentfacevalue 1)
    (return false)
    (elif (== _currentfacevalue 2)
      (return false)
      (elif (== _currentfacevalue 3)
        (return false)
        (elif (== _currentfacevalue 4)
          (return false)
          (elif (== _currentfacevalue 5)
            (return false)
            (elif (== _currentfacevalue 6)
              (return false)
              (else
                (return true)))))))))

(fn `OnCurrentCombinationChanged`
  (params (CurrentCombination :type "/Game/Core/Common/Enums/E_Combinations Enum" :default "NewEnumerator6"))
  (if (`self.IsDiceInCombination`)
    (bind _returnvalue (`NiagaraFunctionLibrary.SpawnSystemAtLocation` "/Game/VFX/Dices/NS_Dice_InCombination.NS_Dice_InCombination" (`SceneComponent.K2_GetComponentLocation` (`self.SM_Dice`))))
    (set `self.NS_DiceInCombination` _returnvalue)
    (else
      (`/Engine/EditorBlueprintResources/StandardMacros.IsValid` (`self.NS_DiceInCombination`)
        (:`Is Valid`
          (`ActorComponent.K2_DestroyComponent` (`self.NS_DiceInCombination`)))))))

(fn `ProcessSpawn`
  (bind _doesoverlap (`self.VerifyOverlappingOtherDices` :!label _label))
  (if _doesoverlap
    (`KismetSystemLibrary.PrintString` "READJUST")
    (`self.AdjustSpawnTransformAndRetry`)
    (goto _label)
    (else
      (`KismetSystemLibrary.PrintString` "OK")
      (set `self.InitialRotation` (`KismetMathLibrary.Conv_RotatorToQuaternion` (`SceneComponent.K2_GetComponentRotation` (`self.SM_Dice`)))))))

(fn `ResetDice`
  (bind _sm_dice (`self.SM_Dice`))
  (`self.ResetSelection`)
  (`PrimitiveComponent.SetAngularDamping` _sm_dice 0.0)
  (`PrimitiveComponent.SetLinearDamping` _sm_dice 0.0)
  (set `self.IsStopped` false)
  (set `self.CurrentFaceValue` 0))

(fn `ResetSelection`
  (`MeshComponent.SetOverlayMaterial` (`self.SM_Dice`) null)
  (set `self.IsSelected` false))

(fn `SpawnDiceVFX`
  (bind (_returnvalue_x _returnvalue_y _returnvalue_z) (`KismetMathLibrary.BreakVector` (`SceneComponent.K2_GetComponentLocation` (`self.SM_Dice`))))
  (bind (_returnvalue_x_2 _returnvalue_y_2 _returnvalue_z_2) (`KismetMathLibrary.BreakVector` (`SceneComponent.K2_GetComponentLocation` (`self.SM_Dice`))))
  (`/Engine/EditorBlueprintResources/StandardMacros.IsValid` (`self.NS_DiceAOE`)
    (:`Is Valid`
      _)
    (:`Is Not Valid`
      (bind _returnvalue (`NiagaraFunctionLibrary.SpawnSystemAtLocation` "/Game/VFX/Dices/NS_Dice_AOE.NS_Dice_AOE" (`KismetMathLibrary.MakeVector` _returnvalue_x_2 _returnvalue_y_2 (- _returnvalue_z_2 3.0))))
      (set `self.NS_DiceAOE` _returnvalue)))
  (`NiagaraComponent.SetVariableFloat` (`self.NS_DiceAOE`) "MaxScale" (select `int` (`self.GetFaceRealValue`) :`0` 0.0 :`1` 50.0 :`2` 55.0 :`3` 60.0 :`4` 65.0 :`5` 72.0 :`6` 80.0 :!type "Float (single-precision)"))
  (`ActorComponent.Activate` (`self.NS_DiceAOE`) true)
  (if (and (not (== (`self.DiceIcon`) "/Game/Assets/2D/UI/Textures/T_Icon_Dice_Basic.T_Icon_Dice_Basic")) (`self.IsPersonaFace`))
    (bind _returnvalue_2 (`GameplayStatics.SpawnDecalAtLocation` "/Game/Materials/M_Decal_DestinationArea.M_Decal_DestinationArea" (8.0 32.0 32.0) (`KismetMathLibrary.MakeVector` _returnvalue_x _returnvalue_y (- _returnvalue_z 3.0)) (struct :`Pitch` -90.0 :`Yaw` -90.0)))
    (set `self.DiceDecal` _returnvalue_2)
    (bind _returnvalue_3 (`KismetMaterialLibrary.CreateDynamicMaterialInstance` "/Game/Materials/M_Decal_DiceAOE.M_Decal_DiceAOE" "None" "Transient"))
    (`MaterialInstanceDynamic.SetTextureParameterValue` _returnvalue_3 "DiceTexture" (`self.DiceIcon`))
    (`DecalComponent.SetDecalMaterial` (`self.DiceDecal`) _returnvalue_3)))

(fn `StopDice`
  (bind (_returnvalue_x _returnvalue_y _returnvalue_z) (`KismetMathLibrary.BreakVector` (`SceneComponent.K2_GetComponentLocation` (`self.SM_Dice`))))
  (`PrimitiveComponent.SetPhysicsAngularVelocityInDegrees` (`self.SM_Dice`) (0.0 0.0 0.0) false "None")
  (`PrimitiveComponent.SetPhysicsLinearVelocity` (`self.SM_Dice`) (0.0 0.0 0.0) false "None")
  (set `self.IsStopped` true)
  (`self.FindFaceValue`)
  (`SceneComponent.K2_SetWorldTransform` (`self.W_DiceValue`) (`KismetMathLibrary.MakeTransform` (`KismetMathLibrary.MakeVector` (- _returnvalue_x 10.0) _returnvalue_y (+ _returnvalue_z 15.0)) (struct) (0.2 0.2 0.2)) false true)
  (bind _asw_dice_value (cast `/Game/Core/UI/W_DiceValue` (`WidgetComponent.GetWidget` (`self.W_DiceValue`))))
  (`/Game/Core/UI/W_DiceValue.UpdateValue` _asw_dice_value (`self.CurrentFaceValue`))
  (if (`self.IsPersonaDice`)
    (`/Game/Core/UI/W_DiceValue.DisplayDiceIcon` _asw_dice_value (`self.PersonaID`))))

(fn `ToggleSelection`
  (if (`self.IsSelected`)
    (`MeshComponent.SetOverlayMaterial` (`self.SM_Dice`) null)
    (set `self.IsSelected` false)
    (`BlueprintMapLibrary.Map_Add` (`/Game/Core/Player/BP_PlayerCharacter.SpawnedDices` (`/Game/Core/Common/Helpers/BFL_Getters.GetMTPlayerCharacter`)) self 1)
    (else
      (`MeshComponent.SetOverlayMaterial` (`self.SM_Dice`) "/Game/Materials/M_Outline_SelectedDice.M_Outline_SelectedDice")
      (set `self.IsSelected` true)
      (`BlueprintMapLibrary.Map_Add` (`/Game/Core/Player/BP_PlayerCharacter.SpawnedDices` (`/Game/Core/Common/Helpers/BFL_Getters.GetMTPlayerCharacter`)) self 2))))

(fn `UpdateDiceCollision`
  (bind (_returnvalue_x _returnvalue_y _returnvalue_z) (`KismetMathLibrary.BreakVector` (`SceneComponent.K2_GetComponentLocation` (`self.SM_Dice`))))
  (`SceneComponent.K2_SetWorldLocation` (`self.DiceAOECollision`) (`KismetMathLibrary.MakeVector` _returnvalue_x _returnvalue_y (- _returnvalue_z 3.0)) false true)
  (`SphereComponent.SetSphereRadius` (`self.DiceAOECollision`) (/ (select `int` (`self.GetFaceRealValue`) :`0` 0.0 :`1` 50.0 :`2` 55.0 :`3` 60.0 :`4` 65.0 :`5` 72.0 :`6` 80.0 :!type "Float (single-precision)") 2.0) true))

(fn `UserConstructionScript`)

(fn `VerifyOverlappingOtherDices`
  (returns (DoesOverlap :type Boolean))
  (bind (_outactors _returnvalue) (`KismetSystemLibrary.BoxOverlapActors` (`SceneComponent.K2_GetComponentLocation` (`self.SM_Dice`)) (2.0 2.0 2.0) (`|MakeArray` "ObjectTypeQuery8" :!type "EObjectTypeQuery Enum") null (`|MakeArray` self :!type "Actor Object Reference")))
  (return _returnvalue))