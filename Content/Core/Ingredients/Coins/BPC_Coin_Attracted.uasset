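; Component that pulls a coin toward the die attracting it and cashes it in for score.
; BeginPlay registers the coin with the game state and computes a flattened XY direction once, which Tick applies as an unswept offset scaled by AmplificationForce.
; When the coin is close to the die, it adds score from face value and coin multiplier.
; It then broadcasts OnCoinCashedIn and destroys the coin and itself.
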(event `self.ReceiveBeginPlay`
  (`self.DoBindings`)
  (`KismetArrayLibrary.Array_Add` (`/Game/Core/Game/BP_GameState.AttractedCoins` (`/Game/Core/Common/Helpers/BFL_Getters.GetMTGameState`)) (`self.AttractedCoin`))
  (`self.CalculateAttractionDirection`))

(event `self.ReceiveTick`
  (params (DeltaSeconds :type "Float (single-precision)"))
  (`self.ProcessAttraction`)
  (if (`self.IsCoinCloseToDice`)
    (`/Game/Core/Game/BP_GameState.UpdateGlobalScore` (`/Game/Core/Common/Helpers/BFL_Getters.GetMTGameState`) (`self.CalculateScore`) (`self.AttractingDice`))
    (`self.CashInCoin`)))

(event `DoBindings`
  (add `self.OnCoinCashedIn` (`|CreateDelegate` (`/Game/Core/Common/Helpers/BFL_Getters.GetMTGameState`) :!event `OnCoinCashedIn`)))

(fn `CalculateAttractionDirection`
  (bind (_returnvalue_x _returnvalue_y) (`KismetMathLibrary.BreakVector` (`KismetMathLibrary.Normal` (- (`SceneComponent.K2_GetComponentLocation` (`/Game/Core/Ingredients/Dices/BP_Dice.SM_Dice` (`self.AttractingDice`))) (`SceneComponent.K2_GetComponentLocation` (`/Game/Core/Ingredients/Coins/BP_Coin_Base.SM_Coin` (`self.AttractedCoin`)))))))
  (set `self.AttractionDirection` (`KismetMathLibrary.MakeVector` _returnvalue_x _returnvalue_y)))

(fn `CalculateScore`
  (returns (ScoreToAdd :type "Float (double-precision)"))
  (return (* (`KismetMathLibrary.Conv_IntToDouble` (* (`/Game/Core/Ingredients/Dices/BP_Dice.GetFaceRealValue` (`self.AttractingDice`)) (`/Game/Core/Ingredients/Coins/BP_Coin_Base.CurrentMultiplier` (`self.AttractedCoin`)))) 10.0)))

(fn `CashInCoin`
  (`self.OnCoinCashedIn` (`self.AttractedCoin`))
  (`Actor.K2_DestroyActor` (`self.AttractedCoin`))
  (`self.K2_DestroyComponent`))

(fn `IsCoinCloseToDice`
  (returns (True :type Boolean))
  (return (<= (`KismetMathLibrary.Vector_Distance` (`SceneComponent.K2_GetComponentLocation` (`/Game/Core/Ingredients/Dices/BP_Dice.SM_Dice` (`self.AttractingDice`))) (`SceneComponent.K2_GetComponentLocation` (`/Game/Core/Ingredients/Coins/BP_Coin_Base.SM_Coin` (`self.AttractedCoin`)))) 10.0)))

(fn `ProcessAttraction`
  (`SceneComponent.K2_AddWorldOffset` (`/Game/Core/Ingredients/Coins/BP_Coin_Base.SM_Coin` (`self.AttractedCoin`)) (* (`self.AttractionDirection`) (`self.AmplificationForce`)) false false))