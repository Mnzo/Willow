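; Base physics coin that drops with a random spin once spawned and reports when it comes to rest.
; OnPostSpawned enables collision and launches it, then Tick watches linear and angular velocity to sleep the body and fire OnCoinStoppedMoving.
; AmplifyCoin looks up a multiplier from the player's map by die face and tints the dynamic material from gold toward red.
; ForcePushbackOnDiceCollision provides an upward impulse scaled by delta time.
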(event `self.ReceiveBeginPlay`
  (`self.CreateDMIMaterials`)
  (`self.DoBindings`))

(event `self.ReceiveTick`
  (params (DeltaSeconds :type "Float (single-precision)"))
  (`|ExecutionSequence`
    (:`then_0`
      (if (`self.IsCoinPhysicallyStopped`)
        (`self.StopCoin`)))))

(event `DoBindings`
  (add `self.OnCoinStoppedMoving` (`|CreateDelegate` (`/Game/Core/Common/Helpers/BFL_Getters.GetMTGameState`) :!event `OnCoinStoppedMoving`)))

(fn `ActivateCollision`
  (`PrimitiveComponent.SetCollisionProfileName` (`self.SM_Coin`) "Coin" true))

(fn `AddInitialMovement`
  (`PrimitiveComponent.SetPhysicsLinearVelocity` (`self.SM_Coin`) (0.0 0.0 -800.0) true "None")
  (`PrimitiveComponent.AddAngularImpulseInDegrees` (`self.SM_Coin`) (* (`KismetMathLibrary.RandomFloatInRange` 360.0 720.0) (`KismetMathLibrary.RandomUnitVector`) 4.0) "None" true))

(fn `AmplifyCoin`
  (params (AmplifyingDice :type "/Game/Core/Ingredients/Dices/BP_Dice Object Reference"))
  (bind _output_get (set `self.CurrentMultiplier` (`BlueprintMapLibrary.Map_Find` (`/Game/Core/Player/BP_PlayerCharacter.MultiplierMap` (`/Game/Core/Common/Helpers/BFL_Getters.GetMTPlayerCharacter`)) (`/Game/Core/Ingredients/Dices/BP_Dice.GetFaceRealValue` AmplifyingDice))))
  (`MaterialInstanceDynamic.SetVectorParameterValue` (`self.DMI_Coin`) "Color" (`KismetMathLibrary.LinearColorLerp` (struct :`R` 0.83077 :`G` 0.723055 :`B` 0.020289 :`A` 1.0) (struct :`R` 1.0 :`B` 0.00761 :`A` 1.0) (`KismetMathLibrary.MapRangeClamped` _output_get 1.0 5.0 0.0 1.0))))

(fn `CreateDMIMaterials`
  (bind _returnvalue (`KismetMaterialLibrary.CreateDynamicMaterialInstance` "/Game/Assets/3D/Ingredients/M_Coin.M_Coin"))
  (bind _output_get (set `self.DMI_Coin` _returnvalue))
  (`PrimitiveComponent.SetMaterial` (`self.SM_Coin`) 0 _output_get))

(fn `ForcePushbackOnDiceCollision`
  (`PrimitiveComponent.AddImpulse` (`self.SM_Coin`) (`KismetMathLibrary.MakeVector` 0.0 0.0 (* (`GameplayStatics.GetWorldDeltaSeconds`) 1000.0)) "None" true))

(fn `IsCoinPhysicallyStopped`
  (returns (True :type Boolean))
  (bind _sm_coin (`self.SM_Coin`))
  (bind _returnvalue (`PrimitiveComponent.GetPhysicsLinearVelocity` _sm_coin "None"))
  (return (and (< (`KismetMathLibrary.VSize` (`PrimitiveComponent.GetPhysicsAngularVelocityInDegrees` _sm_coin "None")) 10.0) (not (`self.IsStopped`)) (`self.IsSpawned`) (< (`KismetMathLibrary.VSize` _returnvalue) 15.0))))

(fn `OnPostSpawned`
  (`self.ActivateCollision`)
  (`self.AddInitialMovement`)
  (set `self.IsSpawned` true))

(fn `StopCoin`
  (`PrimitiveComponent.PutRigidBodyToSleep` (`self.SM_Coin`) "None")
  (set `self.IsStopped` true)
  (`self.OnCoinStoppedMoving`))

(fn `UserConstructionScript`)