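; BP_GameBoard is the clickable game board that the player selects to start playing.
; Clicking while the player is idle moves the game state to pre-throw and the player to playing; further clicks during pre-throw have the player character spawn a destination.
; Hovering while idle shows an outline via overlay material.
; ToggleVisualLimits swaps a mesh material slot to mark the board as unclickable.
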(event `/Game/Core/Common/Interfaces/BPI_ClickableObject.OnClickStart`
  (if (== (`/Game/Core/Player/BP_PlayerCharacter.CurrentState` (`/Game/Core/Common/Helpers/BFL_Getters.GetMTPlayerCharacter`)) "/Game/Core/Player/States/BPC_PlayerState_Idle.BPC_PlayerState_Idle_C")
    (`/Game/Core/Game/BP_GameState.ChangeState` (`/Game/Core/Common/Helpers/BFL_Getters.GetMTGameState`) "/Game/Core/Game/States/BPC_GameState_GB_PreThrow.BPC_GameState_GB_PreThrow_C")
    (`/Game/Core/Player/BP_PlayerCharacter.ChangeState` (`/Game/Core/Common/Helpers/BFL_Getters.GetMTPlayerCharacter`) "/Game/Core/Player/States/BPC_PlayerState_Playing.BPC_PlayerState_Playing_C")
    (`MeshComponent.SetOverlayMaterial` (`self.SM_GameBoard`) null)
    (elif (== (`/Game/Core/Game/BP_GameState.CurrentState` (`/Game/Core/Common/Helpers/BFL_Getters.GetMTGameState`)) "/Game/Core/Game/States/BPC_GameState_GB_PreThrow.BPC_GameState_GB_PreThrow_C")
      (`/Game/Core/Player/BP_PlayerCharacter.SpawnDestination` (`/Game/Core/Common/Helpers/BFL_Getters.GetMTPlayerCharacter`)))))

(event `/Game/Core/Common/Interfaces/BPI_ClickableObject.OnHoveredStart`
  (if (== (`/Game/Core/Player/BP_PlayerCharacter.CurrentState` (`/Game/Core/Common/Helpers/BFL_Getters.GetMTPlayerCharacter`)) "/Game/Core/Player/States/BPC_PlayerState_Idle.BPC_PlayerState_Idle_C")
    (`MeshComponent.SetOverlayMaterial` (`self.SM_GameBoard`) "/Game/Materials/M_Outline.M_Outline")))

(event `/Game/Core/Common/Interfaces/BPI_ClickableObject.OnHoveredEnd`
  (if (== (`/Game/Core/Player/BP_PlayerCharacter.CurrentState` (`/Game/Core/Common/Helpers/BFL_Getters.GetMTPlayerCharacter`)) "/Game/Core/Player/States/BPC_PlayerState_Idle.BPC_PlayerState_Idle_C")
    (`MeshComponent.SetOverlayMaterial` (`self.SM_GameBoard`) null)))

(fn `ToggleVisualLimits`
  (params (ActiveLimits :type Boolean))
  (if ActiveLimits
    (`PrimitiveComponent.SetMaterial` (`self.SM_GameBoard`) 1 "/Game/Assets/3D/Environment/Materials/M_CantClickGameBoard.M_CantClickGameBoard")
    (else
      (`PrimitiveComponent.SetMaterial` (`self.SM_GameBoard`) 1 "/Game/Assets/3D/Environment/Materials/M_GameBoard.M_GameBoard"))))

(fn `UserConstructionScript`)