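; BP_Bell is a clickable bell that can summon the monster when no monster is currently spawned.
; Each click rolls a random number, giving roughly a one-in-five chance to call SpawnMonster on the game state.
; Hovering while the player is in the idle state shows a small-object outline overlay on the bell mesh, unless a monster is already out, and unhovering clears it.
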(event `/Game/Core/Common/Interfaces/BPI_ClickableObject.OnClickStart`
  (if (not (`/Game/Core/Game/BP_GameState.MonsterSpawned` (`/Game/Core/Common/Helpers/BFL_Getters.GetMTGameState`)))
    (if (>= (`KismetMathLibrary.RandomFloatInRange` 0.0 100.0) 80.0)
      (`/Game/Core/Game/BP_GameState.SpawnMonster` (`/Game/Core/Common/Helpers/BFL_Getters.GetMTGameState`)))))

(event `/Game/Core/Common/Interfaces/BPI_ClickableObject.OnHoveredStart`
  (set `self.IsBeingHovered` true)
  (if (and (== (`/Game/Core/Player/BP_PlayerCharacter.CurrentState` (`/Game/Core/Common/Helpers/BFL_Getters.GetMTPlayerCharacter`)) "/Game/Core/Player/States/BPC_PlayerState_Idle.BPC_PlayerState_Idle_C") (not (`/Game/Core/Game/BP_GameState.MonsterSpawned` (`/Game/Core/Common/Helpers/BFL_Getters.GetMTGameState`))))
    (`self.EnableOverlayMaterial`)))

(event `/Game/Core/Common/Interfaces/BPI_ClickableObject.OnHoveredEnd`
  (set `self.IsBeingHovered` false)
  (if (== (`/Game/Core/Player/BP_PlayerCharacter.CurrentState` (`/Game/Core/Common/Helpers/BFL_Getters.GetMTPlayerCharacter`)) "/Game/Core/Player/States/BPC_PlayerState_Idle.BPC_PlayerState_Idle_C")
    (`self.DisableOverlayMaterial`)))

(fn `DisableOverlayMaterial`
  (`MeshComponent.SetOverlayMaterial` (`self.SM_Bell`) null))

(fn `EnableOverlayMaterial`
  (`MeshComponent.SetOverlayMaterial` (`self.SM_Bell`) "/Game/Materials/M_Outline_SmallObject.M_Outline_SmallObject"))

(fn `UserConstructionScript`)