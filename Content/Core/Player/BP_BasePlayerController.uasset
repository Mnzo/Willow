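; Base player controller that sets up Enhanced Input and the root UI for the player.
; On BeginPlay it adds the default mapping context, hides the mouse cursor, then creates the main UI stack widget and adds it to the viewport.
; Tick runs debug and input processing events in sequence, both currently empty.
; A helper returns the current mouse position as a 2D vector.
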(event `self.ReceiveBeginPlay`
  (`self.InitializeInput`)
  (`self.InitializeUI`))

(event `self.ReceiveTick`
  (params (DeltaSeconds :type "Float (single-precision)"))
  (`|ExecutionSequence`
    (:`then_0`
      (`self.ProcessDebugs`))
    (:`then_1`
      (`self.ProcessInputsTick`))))

(event `ProcessDebugs`)

(event `ProcessInputsTick`)

(fn `GetCurrentMousePosition`
  (returns (CurrentClick2DPosition :type "Vector2D Structure"))
  (bind (_locationx _locationy) (`self.GetMousePosition`))
  (return (`KismetMathLibrary.MakeVector2D` _locationx _locationy)))

(fn `InitializeInput`
  (`EnhancedInputSubsystemInterface.AddMappingContext` (subsystem `EnhancedInputLocalPlayerSubsystem`) (`self.DefaultIMC`) 0 (struct))
  (set `self.bShowMouseCursor` false))

(fn `InitializeUI`
  (bind _returnvalue (`|CreateWidget` (`self.DefaultUIStack`)))
  (bind _output_get (set `self.CW_MainStack` _returnvalue))
  (`UserWidget.AddToViewport` _output_get 0))

(fn `UserConstructionScript`)