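; BP_PlayerCharacter is the player character for a dice board game, with wandering between a house and a garden.
; Component-based states, added at runtime, receive tick messages and gate movement and aiming.
; Clicks place decal-marked destinations for saved dice types, then physics throws launch dice along suggested projectile arcs, or to random board points for quick throws.
; A dice-status map drives selective rerolls until the third throw triggers activation.
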(event `self.ReceiveBeginPlay`
  (`self.SaveInitialData`)
  (`self.EnterState` "/Game/Core/Player/States/BPC_PlayerState_Idle.BPC_PlayerState_Idle_C"))

(event `self.ReceiveTick`
  (params (DeltaSeconds :type "Float (single-precision)"))
  (message `/Game/Core/Common/Interfaces/BPI_PlayerStateLogic.OnTick` (`|GetArrayItem` (`self.AllStateObjects`)) DeltaSeconds))

(fn `Aim`
  (params (Yaw :type "Float (double-precision)") (Pitch :type "Float (double-precision)"))
  (if (`/Game/Core/Player/States/BPC_PlayerState_Base.CanMove` (`self.CurrentStateObject`))
    (`self.AddControllerYawInput` (/ Yaw 2.0))
    (`self.AddControllerPitchInput` (/ Pitch 2.0))))

(fn `AreDicesStopped`
  (returns (AllDicesStopped :type Boolean))
  (locals (Stopped :type Boolean))
  (set `local.Stopped` true)
  (bind _keys (`BlueprintMapLibrary.Map_Keys` (`self.SpawnedDices`)))
  (for _array_element _keys
    (if (not (`/Game/Core/Ingredients/Dices/BP_Dice.IsStopped` _array_element))
      (set `local.Stopped` false)
      (break)))
  (return (`local.Stopped`)))

(fn `ChangeState`
  (params (NewState :type "/Game/Core/Player/States/BPC_PlayerState_Base Class Reference"))
  (if (!= NewState (`self.CurrentState`))
    (message `/Game/Core/Common/Interfaces/BPI_PlayerStateLogic.OnExit` (`|GetArrayItem` (`self.AllStateObjects`)))
    (set `self.CurrentState` (`local.NewState`))
    (`self.EnterState` (`self.CurrentState`))))

(fn `DropObject`
  (`self.ChangeState` "/Game/Core/Player/States/BPC_PlayerState_Wandering.BPC_PlayerState_Wandering_C")
  (bind _asbp_homon (cast `/Game/Core/Ingredients/Homonculi/BP_Homon` (`self.LiftedObject`)))
  (set `/Game/Core/Ingredients/Homonculi/BP_Homon.IsBeingLifted` false _asbp_homon)
  (bind _sm_homon (`/Game/Core/Ingredients/Homonculi/BP_Homon.SM_Homon` _asbp_homon))
  (`PrimitiveComponent.SetSimulatePhysics` _sm_homon true)
  (`PrimitiveComponent.AddImpulse` (`/Game/Core/Ingredients/Homonculi/BP_Homon.SM_Homon` _asbp_homon) (* (- (`SceneComponent.K2_GetComponentLocation` _sm_homon) (`self.K2_GetActorLocation`)) 800.0) "None" false)
  (set `self.LiftedObject` null))

(fn `EnterActivation`
  (`PlayerController.SetViewTargetWithBlend` (`/Game/Core/Common/Helpers/BFL_Getters.GetMTGameController`) (`/Game/Core/Game/BP_GameInstance.GetCameraActivation` (`/Game/Core/Common/Helpers/BFL_Getters.GetMTGameInstance`)) 1.5 "VTBlend_EaseOut" 0.2 false))

(fn `EnterGarden`
  (`self.ChangeState` "/Game/Core/Player/States/BPC_PlayerState_Wandering.BPC_PlayerState_Wandering_C")
  (set `CharacterMovementComponent.MaxWalkSpeed` (* (`self.InitialMaxWalkSpeed`) 5.0) (`self.CharacterMovement`))
  (set `self.PreviousHouseTransform` (`KismetMathLibrary.MakeTransform` (`self.K2_GetActorLocation`) (`SceneComponent.K2_GetComponentRotation` (`self.Camera`))))
  (`self.K2_SetActorLocation` (-3500.0 0.0 5100.0) false true)
  (`Controller.SetControlRotation` (`/Game/Core/Common/Helpers/BFL_Getters.GetMTGameController`) (`KismetMathLibrary.MakeRotator` 0.0))
  (bind _outactors (`GameplayStatics.GetAllActorsWithTag` "PPCabin"))
  (bind _aspost_process_volume (cast `PostProcessVolume` (`|GetArrayItem` _outactors)))
  (set `PostProcessVolume.bEnabled` false _aspost_process_volume)
  (bind _outactors_2 (`GameplayStatics.GetAllActorsWithTag` "PPGarden"))
  (bind _aspost_process_volume_2 (cast `PostProcessVolume` (`|GetArrayItem` _outactors_2)))
  (set `PostProcessVolume.bEnabled` true _aspost_process_volume_2))

(fn `EnterHouse`
  (bind (_previoushousetransform_location _previoushousetransform_rotation) (`KismetMathLibrary.BreakTransform` (`self.PreviousHouseTransform`)))
  (bind _returnvalue (== _previoushousetransform_location (0.0 0.0 0.0)))
  (`self.ChangeState` "/Game/Core/Player/States/BPC_PlayerState_Idle.BPC_PlayerState_Idle_C")
  (set `CharacterMovementComponent.MaxWalkSpeed` (`self.InitialMaxWalkSpeed`) (`self.CharacterMovement`))
  (`self.K2_SetActorLocation` (select `bool` _returnvalue :`false` _previoushousetransform_location :`true` (0.0 0.0 95.0)) false true)
  (`Controller.SetControlRotation` (`/Game/Core/Common/Helpers/BFL_Getters.GetMTGameController`) (select `bool` _returnvalue :`false` _previoushousetransform_rotation :`true` (struct :`Yaw` -180.0)))
  (bind _outactors (`GameplayStatics.GetAllActorsWithTag` "PPCabin"))
  (bind _aspost_process_volume (cast `PostProcessVolume` (`|GetArrayItem` _outactors)))
  (set `PostProcessVolume.bEnabled` true _aspost_process_volume)
  (bind _outactors_2 (`GameplayStatics.GetAllActorsWithTag` "PPGarden"))
  (bind _aspost_process_volume_2 (cast `PostProcessVolume` (`|GetArrayItem` _outactors_2)))
  (set `PostProcessVolume.bEnabled` false _aspost_process_volume_2))

(fn `EnterPreThrow`
  (`/Game/Core/UI/CW_PlayerHUD.DeactivateCursor` (`/Game/Core/UI/CW_MainStack.CW_PlayerHUD` (`/Game/Core/Common/Helpers/BFL_Getters.GetCWMainStack`)))
  (`PlayerController.SetViewTargetWithBlend` (`/Game/Core/Common/Helpers/BFL_Getters.GetMTGameController`) (`/Game/Core/Game/BP_GameInstance.GetCameraPreThrow` (`/Game/Core/Common/Helpers/BFL_Getters.GetMTGameInstance`)) 0.2 "VTBlend_Linear" 0.0 false)
  (`KismetSystemLibrary.K2_SetTimer` null "OnCameraPreThrowTransitionFinished" 0.3)
  (set `PlayerController.bShowMouseCursor` true (`/Game/Core/Common/Helpers/BFL_Getters.GetMTGameController`))
  (`/Game/Core/Ingredients/BP_GameBoard.ToggleVisualLimits` (`/Game/Core/Common/Helpers/BFL_Getters.GetGameBoard`) true)
  (`self.ProcessInitialDicesSpawn`))

(fn `EnterState`
  (params (StateToEnter :type "/Game/Core/Player/States/BPC_PlayerState_Base Class Reference"))
  (bind _returnvalue (`|AddComponentByClass` StateToEnter))
  (`KismetArrayLibrary.Array_Add` (`self.AllStateObjects`) _returnvalue)
  (bind _output_get (set `self.CurrentStateObject` _returnvalue))
  (message `/Game/Core/Common/Interfaces/BPI_PlayerStateLogic.OnEnter` _output_get)
  (set `self.CurrentState` (`local.StateToEnter`)))

(fn `EnterThrowing`
  (`PlayerController.SetViewTargetWithBlend` (`/Game/Core/Common/Helpers/BFL_Getters.GetMTGameController`) (`/Game/Core/Game/BP_GameInstance.GetCameraThrowing` (`/Game/Core/Common/Helpers/BFL_Getters.GetMTGameInstance`)) 0.5 "VTBlend_Linear" 0.0 false))

(fn `IsAnyDiceSelected`
  (returns (AtLeastOneSelected :type Boolean))
  (locals (Selected :type Boolean))
  (bind _values (`BlueprintMapLibrary.Map_Values` (`self.SpawnedDices`)))
  (for _array_element _values
    (if (== _array_element 2)
      (set `local.Selected` true)
      (break)
      (else
        (set `local.Selected` false))))
  (return (`local.Selected`)))

(fn `Move`
  (params (`Left/Right` :type "Float (double-precision)") (`Forward/Backward` :type "Float (double-precision)"))
  (if (`/Game/Core/Player/States/BPC_PlayerState_Base.CanMove` (`self.CurrentStateObject`))
    (`self.AddMovementInput` (`self.GetActorRightVector`) `Left/Right`)
    (`self.AddMovementInput` (`self.GetActorForwardVector`) `Forward/Backward`)))

(fn `OnCameraPreThrowTransitionFinished`
  (bind _combinationsnote (`self.CombinationsNote`))
  (`SceneComponent.SetVisibility` (`self.CombinationsNote`) true false)
  (bind _asbp_combinations_note (cast `/Game/Core/Ingredients/BP_CombinationsNote` (`ChildActorComponent.ChildActor` _combinationsnote)))
  (set `/Game/Core/Ingredients/BP_CombinationsNote.InitialPosition` (`SceneComponent.K2_GetComponentLocation` _combinationsnote) _asbp_combinations_note)
  (set `/Game/Core/Ingredients/BP_CombinationsNote.IsAttached` true _asbp_combinations_note))

(fn `PreValidateDices`
  (bind (_keypin _valuepin) (`|MapForEach` (`self.SpawnedDices`))
    (:`then`
      (if (== _valuepin 1)
        (set `/Game/Core/Ingredients/Dices/BP_Dice.IsPreValidated` true _keypin)
        (else
          (set `/Game/Core/Ingredients/Dices/BP_Dice.IsPreValidated` false _keypin))))))

(fn `ProcessDicesAllStopped`
  (if (== (`self.ThrowNumber`) 3)
    (`self.ChangeState` "/Game/Core/Player/States/BPC_PlayerState_Observing.BPC_PlayerState_Observing_C")
    (`/Game/Core/Game/BP_GameState.ChangeState` (`/Game/Core/Common/Helpers/BFL_Getters.GetMTGameState`) "/Game/Core/Game/States/BPC_GameState_GB_Activation.BPC_GameState_GB_Activation_C")
    (else
      (`/Game/Core/Game/BP_GameState.ChangeState` (`/Game/Core/Common/Helpers/BFL_Getters.GetMTGameState`) "/Game/Core/Game/States/BPC_GameState_GB_Evaluating.BPC_GameState_GB_Evaluating_C"))))

(fn `ProcessInitialDicesSpawn`
  (if (== (`self.ThrowNumber`) 0)
    (bind _outactors (`GameplayStatics.GetAllActorsWithTag` "DisplayDices"))
    (for _array_element _outactors
      (`self.SetActorHiddenInGame` _array_element true))
    (for _index (range 5)
      (`self.SpawnDice` _index))))

(fn `QuickThrowDices`
  (locals (Destination :type "Vector Structure") (StartingPoint :type "Vector Structure" :default (0.0 0.0 0.0)) (DiceStaticMesh :type "StaticMeshComponent Object Reference"))
  (bind (_origin _boxextent) (`KismetSystemLibrary.GetComponentBounds` (`/Game/Core/Ingredients/BP_GameBoard.GameBoardQuickThrowZone` (`/Game/Core/Common/Helpers/BFL_Getters.GetGameBoard`))))
  (bind _keys (`BlueprintMapLibrary.Map_Keys` (`self.SpawnedDices`)))
  (for _array_element _keys
    (if (== (`BlueprintMapLibrary.Map_Find` (`self.SpawnedDices`) _array_element) 0)
      (set `/Game/Core/Ingredients/Dices/BP_Dice.IsStopped` false _array_element)
      (`KismetSystemLibrary.K2_SetTimer` _array_element "ActivatePostThrowCollision" 0.5)
      (bind _sm_dice (`/Game/Core/Ingredients/Dices/BP_Dice.SM_Dice` _array_element))
      (set `local.DiceStaticMesh` _sm_dice)
      (set `local.StartingPoint` (`SceneComponent.K2_GetComponentLocation` _sm_dice))
      (set `local.Destination` (`KismetMathLibrary.RandomPointInBoundingBox` _origin _boxextent))
      (`PrimitiveComponent.SetSimulatePhysics` (`local.DiceStaticMesh`) true)
      (bind _outlaunchvelocity (`GameplayStatics.SuggestProjectileVelocity_CustomArc` (`local.StartingPoint`) (`KismetMathLibrary.MakeVector` (.x (`local.Destination`)) (.y (`local.Destination`)) (+ (.z (`local.Destination`)) 10.0))))
      (`PrimitiveComponent.SetPhysicsLinearVelocity` (`local.DiceStaticMesh`) _outlaunchvelocity false "None")
      (`PrimitiveComponent.SetPhysicsAngularVelocityInDegrees` (`local.DiceStaticMesh`) (* (`KismetMathLibrary.RandomFloatInRange` 360.0 720.0) (`KismetMathLibrary.RandomUnitVector`)) false "None")))
  (`self.RemoveAllDestinations`)
  (`/Game/Core/Ingredients/BP_GameBoard.ToggleVisualLimits` (`/Game/Core/Common/Helpers/BFL_Getters.GetGameBoard`) false)
  (bind _keypin (`|MapForEach` (`self.SpawnedDices`))
    (:`then`
      (`BlueprintMapLibrary.Map_Add` (`self.SpawnedDices`) _keypin 1))
    (:`CompletedPin`
      (set `self.ThrowNumber` (+ (`self.ThrowNumber`) 1))
      (`self.ChangeState` "/Game/Core/Player/States/BPC_PlayerState_Adjusting.BPC_PlayerState_Adjusting_C")
      (`/Game/Core/Game/BP_GameState.ChangeState` (`/Game/Core/Common/Helpers/BFL_Getters.GetMTGameState`) "/Game/Core/Game/States/BPC_GameState_GB_Throwing.BPC_GameState_GB_Throwing_C"))))

(fn `RemoveAllDestinations`
  (for _array_element (`self.SpawnedDecals`)
    (`ActorComponent.K2_DestroyComponent` _array_element))
  (`KismetArrayLibrary.Array_Clear` (`self.SpawnedDecals`))
  (`BlueprintMapLibrary.Map_Clear` (`self.DestinationsPositions`))
  (set `self.SpawnedDestinationsNumber` 0))

(fn `RemoveLatestDestination`
  (bind _spawneddecals (`self.SpawnedDecals`))
  (bind _spawneddecals_2 (`self.SpawnedDecals`))
  (if (>= (`self.SpawnedDestinationsNumber`) 1)
    (`ActorComponent.K2_DestroyComponent` (`|GetArrayItem` _spawneddecals (- (`KismetArrayLibrary.Array_Length` _spawneddecals) 1)))
    (`KismetArrayLibrary.Array_Remove` _spawneddecals_2 (- (`KismetArrayLibrary.Array_Length` _spawneddecals_2) 1))
    (bind _keys (`BlueprintMapLibrary.Map_Keys` (`self.DestinationsPositions`)))
    (`BlueprintMapLibrary.Map_Remove` (`self.DestinationsPositions`) (`|GetArrayItem` _keys (`KismetArrayLibrary.Array_LastIndex` _keys)))
    (set `self.SpawnedDestinationsNumber` (- (`self.SpawnedDestinationsNumber`) 1))
    (bind _ascw_pre_throw_hud (cast `/Game/Core/UI/CW_PreThrowHUD` (`CommonActivatableWidgetContainerBase.GetActiveWidget` (`/Game/Core/UI/CW_MainStack.GameStack` (`/Game/Core/Common/Helpers/BFL_Getters.GetCWMainStack`)))))
    (`Widget.SetIsEnabled` (`/Game/Core/UI/CW_PreThrowHUD.ButtonThrow` _ascw_pre_throw_hud) false)))

(fn `RemoveState`
  (params (StateToRemove :type "/Game/Core/Player/States/BPC_PlayerState_Base Object Reference"))
  (bind _statetoremove (`local.StateToRemove`))
  (`KismetArrayLibrary.Array_RemoveItem` (`self.AllStateObjects`) _statetoremove)
  (`ActorComponent.K2_DestroyComponent` _statetoremove))

(fn `ResetSelectedDices`
  (locals (AffectedDices :type "Array of /Game/Core/Ingredients/Dices/BP_Dice Object Reference"))
  (bind _dicesspawnzone (`/Game/Core/Player/Cameras/BP_PlayerCamera_PreThrow.DicesSpawnZone` (cast `/Game/Core/Player/Cameras/BP_PlayerCamera_PreThrow` (`/Game/Core/Game/BP_GameInstance.GetCameraPreThrow` (`/Game/Core/Common/Helpers/BFL_Getters.GetMTGameInstance`)) :!pure true)))
  (bind (_keypin _valuepin) (`|MapForEach` (`self.SpawnedDices`))
    (:`then`
      (if (== _valuepin 2)
        (`KismetArrayLibrary.Array_Add` (`local.AffectedDices`) _keypin)))
    (:`CompletedPin`
      (for _array_element (`local.AffectedDices`)
        (`/Game/Core/Ingredients/Dices/BP_Dice.ResetDice` _array_element)
        (`SceneComponent.K2_SetWorldLocationAndRotation` (`/Game/Core/Ingredients/Dices/BP_Dice.SM_Dice` _array_element) (`KismetMathLibrary.RandomPointInBoundingBox` (`SceneComponent.K2_GetComponentLocation` _dicesspawnzone) (`BoxComponent.BoxExtent` _dicesspawnzone)) (`KismetMathLibrary.RandomRotator` false) false true)
        (`PrimitiveComponent.SetSimulatePhysics` (`/Game/Core/Ingredients/Dices/BP_Dice.SM_Dice` _array_element) false)
        (`BlueprintMapLibrary.Map_Add` (`self.SpawnedDices`) _array_element)))))

(fn `RespawnSelectedDices`
  (`self.PreValidateDices`)
  (`self.ResetSelectedDices`)
  (`/Game/Core/Game/BP_GameState.ChangeState` (`/Game/Core/Common/Helpers/BFL_Getters.GetMTGameState`) "/Game/Core/Game/States/BPC_GameState_GB_PreThrow.BPC_GameState_GB_PreThrow_C")
  (`self.ChangeState` (`/Game/Core/Common/Helpers/BFL_Getters.GetMTPlayerCharacter`) "/Game/Core/Player/States/BPC_PlayerState_Playing.BPC_PlayerState_Playing_C"))

(fn `SaveInitialData`
  (set `self.InitialMaxWalkSpeed` (`CharacterMovementComponent.MaxWalkSpeed` (`self.CharacterMovement`))))

(fn `SelectDice`
  (params (Dice :type "/Game/Core/Ingredients/Dices/BP_Dice Object Reference"))
  (`/Game/Core/Ingredients/Dices/BP_Dice.ToggleSelection` Dice)
  (if (`self.IsAnyDiceSelected`)
    (bind _ascw_evaluating_hud (cast `/Game/Core/UI/CW_EvaluatingHUD` (`CommonActivatableWidgetContainerBase.GetActiveWidget` (`/Game/Core/UI/CW_MainStack.GameStack` (`/Game/Core/Common/Helpers/BFL_Getters.GetCWMainStack`)))))
    (`Widget.SetIsEnabled` (`/Game/Core/UI/CW_EvaluatingHUD.ButtonChange` _ascw_evaluating_hud) true)
    (else
      (bind _ascw_evaluating_hud_2 (cast `/Game/Core/UI/CW_EvaluatingHUD` (`CommonActivatableWidgetContainerBase.GetActiveWidget` (`/Game/Core/UI/CW_MainStack.GameStack` (`/Game/Core/Common/Helpers/BFL_Getters.GetCWMainStack`)))))
      (`Widget.SetIsEnabled` (`/Game/Core/UI/CW_EvaluatingHUD.ButtonChange` _ascw_evaluating_hud_2) false))))

(fn `SpawnDestination`
  (locals (LatestSpawnedDecal :type "DecalComponent Object Reference") (AffectedDice :type "/Game/Core/Ingredients/Dices/BP_Dice Object Reference") (CanContinue :type Boolean) (DicesToThrow :type Integer))
  (bind (_firstclickposition_x _firstclickposition_y _firstclickposition_z) (`KismetMathLibrary.BreakVector` (`/Game/Core/Player/BP_PlayerController_Game.FirstClickPosition` (`/Game/Core/Common/Helpers/BFL_Getters.GetMTGameController`))))
  ;[1 1 1] Throwing conditions: GameBoard's limits
  (if (and (<= _firstclickposition_x -140.0) (<= _firstclickposition_z 112.0))
    (bind (_keypin _valuepin) (`|MapForEach` (`self.SpawnedDices`) :!label _label)
      (:`then`
        (if (and (== _valuepin 0) (not (`.ReturnValue` (`BlueprintMapLibrary.Map_Find` (`self.DestinationsPositions`) _keypin))))
          (set `local.AffectedDice` _keypin)
          (set `local.CanContinue` true)
          (goto _label :!via `BreakPin`)
          (else
            (set `local.CanContinue` false))))
      (:`CompletedPin`
        (if (`local.CanContinue`)
          (`BlueprintMapLibrary.Map_Add` (`self.DestinationsPositions`) (`local.AffectedDice`) (`/Game/Core/Player/BP_PlayerController_Game.FirstClickPosition` (`/Game/Core/Common/Helpers/BFL_Getters.GetMTGameController`)))
          (bind _returnvalue (`GameplayStatics.SpawnDecalAtLocation` "/Game/Materials/M_Decal_DestinationArea.M_Decal_DestinationArea" (8.0 16.0 16.0) (`BlueprintMapLibrary.Map_Find` (`self.DestinationsPositions`) (`local.AffectedDice`)) (`KismetMathLibrary.MakeRotFromX` (`/Game/Core/Player/BP_PlayerController_Game.FirstClickNormal` (`/Game/Core/Common/Helpers/BFL_Getters.GetMTGameController`)))))
          (set `local.LatestSpawnedDecal` _returnvalue)
          (if (> (.y (`/Game/Core/Player/BP_PlayerController_Game.FirstClickNormal` (`/Game/Core/Common/Helpers/BFL_Getters.GetMTGameController`))) 0.5)
            ;[1 1 1] Right GameBoard's border
            (`SceneComponent.K2_SetWorldRotation` (`local.LatestSpawnedDecal`) (struct :`Pitch` -45.0 :`Yaw` 270.0) false false)
            (elif (`/Game/Core/Player/BP_PlayerController_Game.IsFirstClickPlanar` (`/Game/Core/Common/Helpers/BFL_Getters.GetMTGameController`))
              ;[1 1 1] Planar zone
              (`SceneComponent.K2_AddWorldRotation` (`local.LatestSpawnedDecal`) (struct :`Yaw` -90.0 :`Roll` 180.0) false false)
              (else
                ;[1 1 1] Left GameBoard's border
                (`SceneComponent.K2_SetWorldRotation` (`local.LatestSpawnedDecal`) (`KismetMathLibrary.MakeRotator` 0.0 -90.0 -90.0) false false))))
          (bind _returnvalue_2 (`KismetMaterialLibrary.CreateDynamicMaterialInstance` "/Game/Materials/M_Decal_DestinationArea.M_Decal_DestinationArea" "None" "Transient"))
          (`MaterialInstanceDynamic.SetTextureParameterValue` _returnvalue_2 "DiceTexture" (`/Game/Core/Ingredients/Dices/BP_Dice.DiceIcon` (`local.AffectedDice`)))
          (`DecalComponent.SetDecalMaterial` (`local.LatestSpawnedDecal`) _returnvalue_2)
          (`KismetArrayLibrary.Array_Add` (`self.SpawnedDecals`) (`local.LatestSpawnedDecal`))
          (bind (_keypin_2 _valuepin_2) (`|MapForEach` (`self.SpawnedDices`))
            (:`then`
              (if (== _valuepin_2 0)
                (set `local.DicesToThrow` (+ (`local.DicesToThrow`) 1))))
            (:`CompletedPin`
              (bind _output_get (set `self.SpawnedDestinationsNumber` (+ (`self.SpawnedDestinationsNumber`) 1)))
              (if (== _output_get (`local.DicesToThrow`))
                (bind _ascw_pre_throw_hud (cast `/Game/Core/UI/CW_PreThrowHUD` (`CommonActivatableWidgetContainerBase.GetActiveWidget` (`/Game/Core/UI/CW_MainStack.GameStack` (`/Game/Core/Common/Helpers/BFL_Getters.GetCWMainStack`)))))
                (`Widget.SetIsEnabled` (`/Game/Core/UI/CW_PreThrowHUD.ButtonThrow` _ascw_pre_throw_hud) true)))))))))

(fn `SpawnDice`
  (params (DiceID :type Integer))
  (bind _dicesspawnzone (`/Game/Core/Player/Cameras/BP_PlayerCamera_PreThrow.DicesSpawnZone` (cast `/Game/Core/Player/Cameras/BP_PlayerCamera_PreThrow` (`/Game/Core/Game/BP_GameInstance.GetCameraPreThrow` (`/Game/Core/Common/Helpers/BFL_Getters.GetMTGameInstance`)) :!pure true)))
  (bind _returnvalue (`|SpawnActorFromClass` (select `int` (`|GetArrayItem` (`/Game/Core/Game/BP_PlayerSave.DicesTypes` (`/Game/Core/Game/BP_GameInstance.GetSave` (`/Game/Core/Common/Helpers/BFL_Getters.GetMTGameInstance`))) DiceID) :`0` "/Game/Core/Ingredients/Dices/BP_Dice_Basic.BP_Dice_Basic_C" :`1` "/Game/Core/Ingredients/Dices/BP_Dice_No1.BP_Dice_No1_C" :`2` "/Game/Core/Ingredients/Dices/BP_Dice_No2.BP_Dice_No2_C" :`3` "/Game/Core/Ingredients/Dices/BP_Dice_No3.BP_Dice_No3_C" :`4` "/Game/Core/Ingredients/Dices/BP_Dice_No4.BP_Dice_No4_C" :`5` "/Game/Core/Ingredients/Dices/BP_Dice_No5.BP_Dice_No5_C" :!type "Actor Class Reference") (`KismetMathLibrary.MakeTransform` (`KismetMathLibrary.RandomPointInBoundingBox` (`SceneComponent.K2_GetComponentLocation` _dicesspawnzone) (`BoxComponent.BoxExtent` _dicesspawnzone)) (`KismetMathLibrary.RandomRotator` false)) "Undefined" "MultiplyWithRoot" null null))
  (bind _asbp_dice (cast `/Game/Core/Ingredients/Dices/BP_Dice` _returnvalue))
  (`PrimitiveComponent.SetSimulatePhysics` (`/Game/Core/Ingredients/Dices/BP_Dice.SM_Dice` _asbp_dice) false)
  (`BlueprintMapLibrary.Map_Add` (`self.SpawnedDices`) _asbp_dice))

(fn `ThrowDices`
  (locals (Destination :type "Vector Structure") (StartingPoint :type "Vector Structure" :default (0.0 0.0 0.0)) (DiceStaticMesh :type "StaticMeshComponent Object Reference"))
  (bind _keys (`BlueprintMapLibrary.Map_Keys` (`self.SpawnedDices`)))
  (for _array_element _keys
    (if (== (`BlueprintMapLibrary.Map_Find` (`self.SpawnedDices`) _array_element) 0)
      (set `/Game/Core/Ingredients/Dices/BP_Dice.IsStopped` false _array_element)
      (`KismetSystemLibrary.K2_SetTimer` _array_element "ActivatePostThrowCollision" 0.5)
      (bind _sm_dice (`/Game/Core/Ingredients/Dices/BP_Dice.SM_Dice` _array_element))
      (set `local.DiceStaticMesh` _sm_dice)
      (set `local.StartingPoint` (`SceneComponent.K2_GetComponentLocation` _sm_dice))
      (set `local.Destination` (`BlueprintMapLibrary.Map_Find` (`self.DestinationsPositions`) _array_element))
      (`PrimitiveComponent.SetSimulatePhysics` (`local.DiceStaticMesh`) true)
      (bind _outlaunchvelocity (`GameplayStatics.SuggestProjectileVelocity_CustomArc` (`local.StartingPoint`) (`KismetMathLibrary.MakeVector` (.x (`local.Destination`)) (.y (`local.Destination`)) (+ (.z (`local.Destination`)) 10.0))))
      (`PrimitiveComponent.SetPhysicsLinearVelocity` (`local.DiceStaticMesh`) _outlaunchvelocity false "None")
      (`PrimitiveComponent.SetPhysicsAngularVelocityInDegrees` (`local.DiceStaticMesh`) (* (`KismetMathLibrary.RandomFloatInRange` 360.0 720.0) (`KismetMathLibrary.RandomUnitVector`) 0.5) false "None")))
  (`self.RemoveAllDestinations`)
  (`/Game/Core/Ingredients/BP_GameBoard.ToggleVisualLimits` (`/Game/Core/Common/Helpers/BFL_Getters.GetGameBoard`) false)
  (bind _keypin (`|MapForEach` (`self.SpawnedDices`))
    (:`then`
      (`BlueprintMapLibrary.Map_Add` (`self.SpawnedDices`) _keypin 1))
    (:`CompletedPin`
      (set `self.ThrowNumber` (+ (`self.ThrowNumber`) 1))
      (`self.ChangeState` "/Game/Core/Player/States/BPC_PlayerState_Adjusting.BPC_PlayerState_Adjusting_C")
      (`/Game/Core/Game/BP_GameState.ChangeState` (`/Game/Core/Common/Helpers/BFL_Getters.GetMTGameState`) "/Game/Core/Game/States/BPC_GameState_GB_Throwing.BPC_GameState_GB_Throwing_C"))))

(fn `UserConstructionScript`)