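; Game player controller that routes movement, look, eye-closing and click input to the player character, its states and the HUD.
; Clicks and per-tick hover target BPI_ClickableObject actors, using a screen-center trace or a cursor trace depending on the current player state.
; Left click also drops lifted objects or exits UI zoom.
; In the pre-throw game state, right click removes the latest destination and a debug key respawns dice.
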(event `self.ReceiveBeginPlay`
  (`parent.ReceiveBeginPlay`))

(event `EnhancedInput|/Game/Inputs/EnhancedInput/InputActions/IA_CloseEyes`
  (params (ActionValue :type Boolean) (ElapsedSeconds :type "Float (double-precision)") (TriggeredSeconds :type "Float (double-precision)") (InputAction :type "InputAction Object Reference" :default "/Game/Inputs/EnhancedInput/InputActions/IA_CloseEyes.IA_CloseEyes"))
  (:`Started`
    (`/Game/Core/Player/BP_PlayerCharacter.ChangeState` (`/Game/Core/Common/Helpers/BFL_Getters.GetMTPlayerCharacter`) "/Game/Core/Player/States/BPC_PlayerState_EyesTransition.BPC_PlayerState_EyesTransition_C")
    (`/Game/Core/UI/CW_PlayerHUD.StartClosingEyes` (`/Game/Core/UI/CW_MainStack.CW_PlayerHUD` (`self.GetMainStack`)) 2.0))
  (:`Completed`
    (if (== (`/Game/Core/Player/BP_PlayerCharacter.CurrentState` (`/Game/Core/Common/Helpers/BFL_Getters.GetMTPlayerCharacter`)) "/Game/Core/Player/States/BPC_PlayerState_EyesTransition.BPC_PlayerState_EyesTransition_C")
      (`/Game/Core/Player/BP_PlayerCharacter.ChangeState` (`/Game/Core/Common/Helpers/BFL_Getters.GetMTPlayerCharacter`) "/Game/Core/Player/States/BPC_PlayerState_Idle.BPC_PlayerState_Idle_C")
      (`/Game/Core/UI/CW_PlayerHUD.EndClosingEyes` (`/Game/Core/UI/CW_MainStack.CW_PlayerHUD` (`self.GetMainStack`))))))

(event `EnhancedInput|/Game/Inputs/EnhancedInput/InputActions/IA_Move`
  (params (ActionValue :type "Vector2D Structure") (ElapsedSeconds :type "Float (double-precision)") (TriggeredSeconds :type "Float (double-precision)") (InputAction :type "InputAction Object Reference" :default "/Game/Inputs/EnhancedInput/InputActions/IA_Move.IA_Move"))
  ;[1 1 1] Movement inputs
  (:`Triggered`
    (`/Game/Core/Player/BP_PlayerCharacter.Move` (`/Game/Core/Common/Helpers/BFL_Getters.GetMTPlayerCharacter`) ActionValue_X ActionValue_Y)))

(event `EnhancedInput|/Game/Inputs/EnhancedInput/InputActions/IA_LeftClick`
  (params (ActionValue :type Boolean) (ElapsedSeconds :type "Float (double-precision)") (TriggeredSeconds :type "Float (double-precision)") (InputAction :type "InputAction Object Reference" :default "/Game/Inputs/EnhancedInput/InputActions/IA_LeftClick.IA_LeftClick"))
  (bind (_locationx _locationy) (`self.GetMousePosition`))
  (bind _mtplayercharacter (`/Game/Core/Common/Helpers/BFL_Getters.GetMTPlayerCharacter`))
  (bind _clickedactor (`self.ClickedActor`))
  (bind _clickedactor_2 (`self.ClickedActor`))
  (bind (_bblockinghit _binitialoverlap _time _distance _location _impactpoint _normal _impactnormal _physmat _hitactor) (`GameplayStatics.BreakHitResult` (`self.GetHitResultUnderCursorByChannel` "TraceTypeQuery1")))
  (bind (_worldposition _worlddirection) (`GameplayStatics.DeprojectScreenToWorld` self (/ (`WidgetLayoutLibrary.GetViewportSize`) (2.0 2.0))))
  (:`Triggered`
    (`KismetSystemLibrary.PrintString` "IA_LeftClick triggered" true true (struct :`G` 0.66 :`B` 1.0 :`A` 1.0) 0.0)
    (`/Engine/EditorBlueprintResources/StandardMacros.IsValid` _clickedactor_2
      (:`Is Valid`
        (message `/Game/Core/Common/Interfaces/BPI_ClickableObject.OnClickUpdate` _clickedactor_2))))
  (:`Started`
    (`KismetSystemLibrary.PrintString` "IA_LeftClick started")
    (`/Engine/EditorBlueprintResources/StandardMacros.IsValid` (`/Game/Core/Player/BP_PlayerCharacter.CurrentStateObject` (`/Game/Core/Common/Helpers/BFL_Getters.GetMTPlayerCharacter`))
      (:`Is Valid`
        (if (`/Game/Core/Player/States/BPC_PlayerState_Base.IsClickCenteredBase` (`/Game/Core/Player/BP_PlayerCharacter.CurrentStateObject` (`/Game/Core/Common/Helpers/BFL_Getters.GetMTPlayerCharacter`)))
          (if (== (`/Game/Core/Player/BP_PlayerCharacter.CurrentState` (`/Game/Core/Common/Helpers/BFL_Getters.GetMTPlayerCharacter`)) "/Game/Core/Player/States/BPC_PlayerState_Lifting.BPC_PlayerState_Lifting_C")
            (`/Game/Core/Player/BP_PlayerCharacter.DropObject` (`/Game/Core/Common/Helpers/BFL_Getters.GetMTPlayerCharacter`))
            (else
              (bind _outhit (`KismetSystemLibrary.LineTraceSingleForObjects` _worldposition (+ _worldposition (* _worlddirection 1000.0)) (`|MakeArray` "ObjectTypeQuery7" "ObjectTypeQuery10" :!type "EObjectTypeQuery Enum")))
              (bind (_bblockinghit_2 _binitialoverlap_2 _time_2 _distance_2 _location_2 _impactpoint_2 _normal_2 _impactnormal_2 _physmat_2 _hitactor_2) (`GameplayStatics.BreakHitResult` _outhit))
              (if (`KismetSystemLibrary.DoesImplementInterface` _hitactor_2 "/Game/Core/Common/Interfaces/BPI_ClickableObject.BPI_ClickableObject_C")
                (bind _output_get (set `self.ClickedActor` _hitactor_2))
                (message `/Game/Core/Common/Interfaces/BPI_ClickableObject.OnClickStart` _output_get))))
          (elif (`self.InputsActive`)
            (if (== (`/Game/Core/Player/BP_PlayerCharacter.CurrentState` (`/Game/Core/Common/Helpers/BFL_Getters.GetMTPlayerCharacter`)) "/Game/Core/Player/States/BPC_PlayerState_UIZooming.BPC_PlayerState_UIZooming_C")
              (`/Game/Core/Ingredients/BP_CombinationsNote.StopCenteringBehavior` (`/Game/Core/Player/BP_PlayerCharacter.GetCombinationsNoteBP` (`/Game/Core/Common/Helpers/BFL_Getters.GetMTPlayerCharacter`)))
              (`/Game/Core/Player/BP_PlayerCharacter.ChangeState` _mtplayercharacter (`/Game/Core/Player/BP_PlayerCharacter.PreviousState` _mtplayercharacter))
              (elif (`KismetSystemLibrary.DoesImplementInterface` _hitactor "/Game/Core/Common/Interfaces/BPI_ClickableObject.BPI_ClickableObject_C")
                (bind _output_get_2 (set `self.ClickedActor` _hitactor))
                (set `self.FirstClickPosition` _location)
                (set `self.FirstClickNormal` _normal)
                (set `self.FirstClick2DPosition` (`KismetMathLibrary.MakeVector2D` _locationx _locationy))
                (message `/Game/Core/Common/Interfaces/BPI_ClickableObject.OnClickStart` _output_get_2))))))))
  (:`Completed`
    (`KismetSystemLibrary.PrintString` "IA_LeftClick completed" true true (struct :`G` 0.66 :`B` 1.0 :`A` 1.0) 0.0)
    (`/Engine/EditorBlueprintResources/StandardMacros.IsValid` _clickedactor
      (:`Is Valid`
        (message `/Game/Core/Common/Interfaces/BPI_ClickableObject.OnClickStop` _clickedactor)
        (set `self.ClickedActor` null)))))

(event `EnhancedInput|/Game/Inputs/EnhancedInput/InputActions/IA_Look`
  (params (ActionValue :type "Vector2D Structure") (ElapsedSeconds :type "Float (double-precision)") (TriggeredSeconds :type "Float (double-precision)") (InputAction :type "InputAction Object Reference" :default "/Game/Inputs/EnhancedInput/InputActions/IA_Look.IA_Look"))
  ;[1 1 1] Movement inputs
  (:`Triggered`
    (`/Game/Core/Player/BP_PlayerCharacter.Aim` (`/Game/Core/Common/Helpers/BFL_Getters.GetMTPlayerCharacter`) (* ActionValue_X 1.5) (* ActionValue_Y 1.5))))

(event `EnhancedInput|/Game/Inputs/EnhancedInput/InputActions/IA_MouseLook`
  (params (ActionValue :type "Vector2D Structure") (ElapsedSeconds :type "Float (double-precision)") (TriggeredSeconds :type "Float (double-precision)") (InputAction :type "InputAction Object Reference" :default "/Game/Inputs/EnhancedInput/InputActions/IA_MouseLook.IA_MouseLook"))
  ;[1 1 1] Movement inputs
  (:`Triggered`
    (`/Game/Core/Player/BP_PlayerCharacter.Aim` (`/Game/Core/Common/Helpers/BFL_Getters.GetMTPlayerCharacter`) ActionValue_X ActionValue_Y)))

(event `EnhancedInput|/Game/Inputs/EnhancedInput/InputActions/IA_RightClick`
  (params (ActionValue :type Boolean) (ElapsedSeconds :type "Float (double-precision)") (TriggeredSeconds :type "Float (double-precision)") (InputAction :type "InputAction Object Reference" :default "/Game/Inputs/EnhancedInput/InputActions/IA_RightClick.IA_RightClick"))
  (:`Started`
    (if (== (`/Game/Core/Game/BP_GameState.CurrentState` (`/Game/Core/Common/Helpers/BFL_Getters.GetMTGameState`)) "/Game/Core/Game/States/BPC_GameState_GB_PreThrow.BPC_GameState_GB_PreThrow_C")
      (`/Game/Core/Player/BP_PlayerCharacter.RemoveLatestDestination` (`/Game/Core/Common/Helpers/BFL_Getters.GetMTPlayerCharacter`)))))

(event `self.ProcessInputsTick`
  (bind (_bblockinghit _binitialoverlap _time _distance _location _impactpoint _normal _impactnormal _physmat _hitactor) (`GameplayStatics.BreakHitResult` (`self.GetHitResultUnderCursorByChannel` "TraceTypeQuery1")))
  (bind (_worldposition _worlddirection) (`GameplayStatics.DeprojectScreenToWorld` self (/ (`WidgetLayoutLibrary.GetViewportSize`) (2.0 2.0))))
  (`parent.ProcessInputsTick`)
  (if (`/Game/Core/Player/States/BPC_PlayerState_Base.IsClickCenteredBase` (`/Game/Core/Player/BP_PlayerCharacter.CurrentStateObject` (`/Game/Core/Common/Helpers/BFL_Getters.GetMTPlayerCharacter`)))
    (bind _outhit (`KismetSystemLibrary.LineTraceSingleForObjects` _worldposition (+ _worldposition (* _worlddirection 1000.0)) (`|MakeArray` "ObjectTypeQuery7" "ObjectTypeQuery10" :!type "EObjectTypeQuery Enum")))
    (bind (_bblockinghit_2 _binitialoverlap_2 _time_2 _distance_2 _location_2 _impactpoint_2 _normal_2 _impactnormal_2 _physmat_2 _hitactor_2) (`GameplayStatics.BreakHitResult` _outhit))
    (if (`KismetSystemLibrary.DoesImplementInterface` _hitactor_2 "/Game/Core/Common/Interfaces/BPI_ClickableObject.BPI_ClickableObject_C")
      (`/Engine/EditorBlueprintResources/StandardMacros.IsValid` (`self.HoveredActor`)
        (:`Is Valid`
          (if (!= _hitactor_2 (`self.HoveredActor`))
            (message `/Game/Core/Common/Interfaces/BPI_ClickableObject.OnHoveredEnd` (`self.HoveredActor`))
            (bind _output_get (set `self.HoveredActor` _hitactor_2))
            (message `/Game/Core/Common/Interfaces/BPI_ClickableObject.OnHoveredStart` _output_get)))
        (:`Is Not Valid`
          (bind _output_get_2 (set `self.HoveredActor` _hitactor_2))
          (message `/Game/Core/Common/Interfaces/BPI_ClickableObject.OnHoveredStart` _output_get_2)))
      (else
        (`/Engine/EditorBlueprintResources/StandardMacros.IsValid` (`self.HoveredActor`)
          (:`Is Valid`
            (message `/Game/Core/Common/Interfaces/BPI_ClickableObject.OnHoveredEnd` (`self.HoveredActor`))
            (set `self.HoveredActor` null)))))
    (elif (`self.InputsActive`)
      (if (`KismetSystemLibrary.DoesImplementInterface` _hitactor "/Game/Core/Common/Interfaces/BPI_ClickableObject.BPI_ClickableObject_C")
        (`/Engine/EditorBlueprintResources/StandardMacros.IsValid` (`self.HoveredActor`)
          (:`Is Valid`
            (if (!= _hitactor (`self.HoveredActor`))
              (message `/Game/Core/Common/Interfaces/BPI_ClickableObject.OnHoveredEnd` (`self.HoveredActor`))
              (bind _output_get_3 (set `self.HoveredActor` _hitactor))
              (message `/Game/Core/Common/Interfaces/BPI_ClickableObject.OnHoveredStart` _output_get_3)))
          (:`Is Not Valid`
            (bind _output_get_4 (set `self.HoveredActor` _hitactor))
            (message `/Game/Core/Common/Interfaces/BPI_ClickableObject.OnHoveredStart` _output_get_4)))
        (else
          (`/Engine/EditorBlueprintResources/StandardMacros.IsValid` (`self.HoveredActor`)
            (:`Is Valid`
              (message `/Game/Core/Common/Interfaces/BPI_ClickableObject.OnHoveredEnd` (`self.HoveredActor`))
              (set `self.HoveredActor` null))))))))

(event `self.ProcessDebugs`
  (`parent.ProcessDebugs`))

(event `Key|L`
  (params (Key :type "Key Structure"))
  (bind _spawneddices (`/Game/Core/Player/BP_PlayerCharacter.SpawnedDices` (`/Game/Core/Common/Helpers/BFL_Getters.GetMTPlayerCharacter`)))
  ;[1 0 0] DEBUG: Rearrange spawned dices
  (:`Pressed`
    (if (== (`/Game/Core/Game/BP_GameState.CurrentState` (`/Game/Core/Common/Helpers/BFL_Getters.GetMTGameState`)) "/Game/Core/Game/States/BPC_GameState_GB_PreThrow.BPC_GameState_GB_PreThrow_C")
      (bind _keypin (`|MapForEach` _spawneddices)
        (:`then`
          (`self.K2_DestroyActor` _keypin))
        (:`CompletedPin`
          (`BlueprintMapLibrary.Map_Clear` _spawneddices)
          (for _index (range 5)
            (`/Game/Core/Player/BP_PlayerCharacter.SpawnDice` (`/Game/Core/Common/Helpers/BFL_Getters.GetMTPlayerCharacter`) _index)))))))

(fn `GetMainStack`
  (returns (MainStack :type "/Game/Core/UI/CW_MainStack Object Reference"))
  (bind _ascw_main_stack (cast `/Game/Core/UI/CW_MainStack` (`self.CW_MainStack`)))
  (return _ascw_main_stack))

(fn `IsFirstClickPlanar`
  (returns (NewParam :type Boolean))
  (bind (_firstclicknormal_x _firstclicknormal_y) (`KismetMathLibrary.BreakVector` (`/Game/Core/Player/BP_PlayerController_Game.FirstClickNormal` (`/Game/Core/Common/Helpers/BFL_Getters.GetMTGameController`))))
  (return (and (> _firstclicknormal_y -0.1) (< _firstclicknormal_y 0.1))))

(fn `ReactivateInputs`
  (bind _output_get (set `self.InputsActive` true))
  (`self.OnInputsActivationToggled` _output_get))

(fn `UserConstructionScript`)