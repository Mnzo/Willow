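; Base player state component, defining the lifecycle events and permission queries for states on the player character.
; Enter, tick and exit events print the state's class name as on-screen debug text, and exit also removes the state from the player character.
; Query functions supply defaults: movement and centered-click are true, while dice rotation, dice selection and Homon selection are false.
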(event `/Game/Core/Common/Interfaces/BPI_PlayerStateLogic.OnEnter`
  (`KismetSystemLibrary.PrintString` (`KismetStringLibrary.Concat_StrStr` "PLAYER STATE ENTERED:   " (`KismetSystemLibrary.GetClassDisplayName` (`GameplayStatics.GetObjectClass` self))) true true (struct :`R` 1.0 :`G` 0.05448 :`B` 0.001821 :`A` 1.0) 5.0))

(event `/Game/Core/Common/Interfaces/BPI_PlayerStateLogic.OnTick`
  (params (DeltaSeconds :type "Float (double-precision)"))
  (`KismetSystemLibrary.PrintString` (`KismetStringLibrary.Concat_StrStr` "CURRENT PLAYER STATE:   " (`KismetSystemLibrary.GetClassDisplayName` (`GameplayStatics.GetObjectClass` self))) true true (struct :`R` 1.0 :`G` 0.05448 :`B` 0.001821 :`A` 1.0) 0.0))

(event `/Game/Core/Common/Interfaces/BPI_PlayerStateLogic.OnExit`
  (`KismetSystemLibrary.PrintString` (`KismetStringLibrary.Concat_StrStr` "PLAYER STATE REMOVED:   " (`KismetSystemLibrary.GetClassDisplayName` (`GameplayStatics.GetObjectClass` self))) true true (struct :`R` 1.0 :`G` 0.05448 :`B` 0.001821 :`A` 1.0) 5.0)
  (`/Game/Core/Player/BP_PlayerCharacter.RemoveState` (`/Game/Core/Common/Helpers/BFL_Getters.GetMTPlayerCharacter`) self))

(fn `CanMove`
  (returns (CanMove :type Boolean))
  (return true))

(fn `CanRotateDices`
  (returns (CanRotateDices :type Boolean))
  (return false))

(fn `CanSelectDices`
  (returns (CanSelectDices :type Boolean))
  (return false))

(fn `CanSelectHomon`
  (returns (CanSelectHomon :type Boolean))
  (return false))

(fn `IsClickCenteredBase`
  (returns (CenteredBaseClick :type Boolean))
  (return true))