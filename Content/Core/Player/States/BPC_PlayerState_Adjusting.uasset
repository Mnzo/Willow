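; Player state component for the Adjusting phase, in which the player can select dice but cannot move or rotate them.
; On BeginPlay it tells the game controller to switch to the throwing camera and deactivate inputs, unless the previous state was UI zooming.
; Query functions return fixed permissions for this state, also disabling click-centered base behavior.
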(event `self.ReceiveBeginPlay`
  (bind _mtgamecontroller (`/Game/Core/Common/Helpers/BFL_Getters.GetMTGameController`))
  (if (not (== (`/Game/Core/Player/BP_PlayerCharacter.PreviousState` (`/Game/Core/Common/Helpers/BFL_Getters.GetMTPlayerCharacter`)) "/Game/Core/Player/States/BPC_PlayerState_UIZooming.BPC_PlayerState_UIZooming_C"))
    (`/Game/Core/Player/BP_PlayerController_Game.SwitchToThrowingCamera` _mtgamecontroller)
    (`/Game/Core/Player/BP_PlayerController_Game.DeactivateInputs` _mtgamecontroller)))

(fn `CanMove`
  (returns (CanMove :type Boolean))
  (return false))

(fn `CanRotateDices`
  (returns (CanRotateDices :type Boolean))
  (return false))

(fn `CanSelectDices`
  (returns (CanSelectDices :type Boolean))
  (return true))

(fn `IsClickCenteredBase`
  (returns (CenteredBaseClick :type Boolean))
  (return false))