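; Player state component for the Playing state of the player character, a phase centred on throwing dice.
; On BeginPlay it puts the character into pre-throw, unless the previous state was UI zooming.
; Its overrides block movement, allow rotating dice and report that clicks are not centre-based.
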(event `self.ReceiveBeginPlay`
  (if (not (== (`/Game/Core/Player/BP_PlayerCharacter.PreviousState` (`/Game/Core/Common/Helpers/BFL_Getters.GetMTPlayerCharacter`)) "/Game/Core/Player/States/BPC_PlayerState_UIZooming.BPC_PlayerState_UIZooming_C"))
    (`/Game/Core/Player/BP_PlayerCharacter.EnterPreThrow` (`/Game/Core/Common/Helpers/BFL_Getters.GetMTPlayerCharacter`))))

(fn `CanMove`
  (returns (CanMove :type Boolean))
  (return false))

(fn `CanRotateDices`
  (returns (CanRotateDices :type Boolean))
  (return true))

(fn `IsClickCenteredBase`
  (returns (CenteredBaseClick :type Boolean))
  (return false))