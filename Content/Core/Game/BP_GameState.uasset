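; Game state Blueprint that runs a component-based state machine, starting in the Idle state after a brief fail-safe delay and HUD transition-in.
; EnterState adds the state class as a component, tracks it and sends its enter message.
; ChangeState sends exit to the first tracked state before entering the new one, while RemoveState separately destroys components.
; Tick prints global time dilation for debugging.
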(event `self.ReceiveBeginPlay`
  ;[1 1 1] Global initializations are made before, it is a fail safe delay before doing the transition visual and actually starting game
  (`KismetSystemLibrary.Delay` 0.2)
  (`/Game/Core/UI/BP_HUD.TransitionIn` (`/Game/Core/Common/Helpers/BFL_Getters.GetMTHUD`))
  (`self.EnterState` "/Game/Core/Game/States/BPC_GameState_Idle.BPC_GameState_Idle_C"))

(event `self.ReceiveTick`
  (params (DeltaSeconds :type "Float (single-precision)"))
  (`|ExecutionSequence`
    (:`then_0`
      (`self.ProcessDebugs`))))

(event `ProcessDebugs`
  (`KismetSystemLibrary.PrintString` (`KismetStringLibrary.Concat_StrStr` "CurrentTimeDilation:   " (`KismetStringLibrary.Conv_DoubleToString` (`GameplayStatics.GetGlobalTimeDilation`)) " \n") true true (struct :`G` 0.84375 :`B` 0.047923 :`A` 1.0) 0.0))

(fn `ChangeState`
  (params (NewState :type "/Game/Core/Game/States/BPC_GameState_Base Class Reference"))
  (if (!= NewState (`self.CurrentState`))
    (message `/Game/Core/Common/Interfaces/BPI_GameStateLogic.OnExit` (`|GetArrayItem` (`self.AllStateObjects`)))
    (set `self.CurrentState` (`local.NewState`))
    (`self.EnterState` (`self.CurrentState`))))

(fn `EnterState`
  (params (StateToEnter :type "/Game/Core/Game/States/BPC_GameState_Base Class Reference"))
  (bind _returnvalue (`|AddComponentByClass` StateToEnter))
  (`KismetArrayLibrary.Array_Add` (`self.AllStateObjects`) _returnvalue)
  (bind _output_get (set `self.CurrentStateObject` _returnvalue))
  (message `/Game/Core/Common/Interfaces/BPI_GameStateLogic.OnEnter` _output_get)
  (set `self.CurrentState` (`local.StateToEnter`)))

(fn `RemoveState`
  (params (StateToRemove :type "/Game/Core/Game/States/BPC_GameState_Base Object Reference"))
  (bind _statetoremove (`local.StateToRemove`))
  (`KismetArrayLibrary.Array_RemoveItem` (`self.AllStateObjects`) _statetoremove)
  (`ActorComponent.K2_DestroyComponent` _statetoremove))

(fn `UserConstructionScript`)