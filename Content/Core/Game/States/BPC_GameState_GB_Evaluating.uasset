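; Game state Blueprint for the evaluating phase, in which the player's spawned dice are shown alongside validate and change options.
; On begin play it pushes the evaluating HUD onto the main widget stack and reactivates controller inputs.
; After a short delay, it reveals the Validate and Change buttons on the active HUD, then forces the hover start on each of the player's spawned dice.
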(event `self.ReceiveBeginPlay`
  (`/Game/Core/UI/CW_MainStack.PushGameStack` (`/Game/Core/Common/Helpers/BFL_Getters.GetCWMainStack`) "/Game/Core/UI/CW_EvaluatingHUD.CW_EvaluatingHUD_C")
  (`/Game/Core/Player/BP_PlayerController_Game.ReactivateInputs` (`/Game/Core/Common/Helpers/BFL_Getters.GetMTGameController`))
  (`KismetSystemLibrary.Delay` 0.5)
  (`self.ShowValidateButton`)
  (`self.ShowChangeButton`)
  (bind _keypin (`|MapForEach` (`/Game/Core/Player/BP_PlayerCharacter.SpawnedDices` (`/Game/Core/Common/Helpers/BFL_Getters.GetMTPlayerCharacter`)))
    (:`then`
      (`/Game/Core/Ingredients/Dices/BP_Dice.ForceHoveredStart` _keypin))))

(fn `ShowChangeButton`
  (bind _ascw_evaluating_hud (cast `/Game/Core/UI/CW_EvaluatingHUD` (`CommonActivatableWidgetContainerBase.GetActiveWidget` (`/Game/Core/UI/CW_MainStack.GameStack` (`/Game/Core/Common/Helpers/BFL_Getters.GetCWMainStack`)))))
  (`Widget.SetVisibility` (`/Game/Core/UI/CW_EvaluatingHUD.ButtonChange` _ascw_evaluating_hud) "Visible"))

(fn `ShowValidateButton`
  (bind _ascw_evaluating_hud (cast `/Game/Core/UI/CW_EvaluatingHUD` (`CommonActivatableWidgetContainerBase.GetActiveWidget` (`/Game/Core/UI/CW_MainStack.GameStack` (`/Game/Core/Common/Helpers/BFL_Getters.GetCWMainStack`)))))
  (`Widget.SetVisibility` (`/Game/Core/UI/CW_EvaluatingHUD.ButtonValidate` _ascw_evaluating_hud) "Visible"))