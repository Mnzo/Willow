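; Base component class for game states, giving child states empty Enter, Tick and Exit functions to override.
; OnEnter, OnTick and OnExit events wrap these hooks and print the state's class name to screen in a different color for each phase.
; OnExit also removes the state from the MT GameState before calling Exit.
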(event `/Game/Core/Common/Interfaces/BPI_GameStateLogic.OnEnter`
  (`KismetSystemLibrary.PrintString` (`KismetStringLibrary.Concat_StrStr` "GAME STATE ENTERED:   " (`KismetSystemLibrary.GetClassDisplayName` (`GameplayStatics.GetObjectClass` self))) true true (struct :`R` 1.0 :`G` 1.0 :`B` 1.0 :`A` 1.0) 5.0)
  (`self.Enter`))

(event `/Game/Core/Common/Interfaces/BPI_GameStateLogic.OnTick`
  (params (DeltaSeconds :type "Float (double-precision)"))
  (`KismetSystemLibrary.PrintString` (`KismetStringLibrary.Concat_StrStr` "CURRENT GAME STATE:   " (`KismetSystemLibrary.GetClassDisplayName` (`GameplayStatics.GetObjectClass` self))) true true (struct :`G` 0.242281 :`B` 1.0 :`A` 1.0) 0.0)
  (`self.Tick`))

(event `/Game/Core/Common/Interfaces/BPI_GameStateLogic.OnExit`
  (`KismetSystemLibrary.PrintString` (`KismetStringLibrary.Concat_StrStr` "GAME STATE REMOVED:   " (`KismetSystemLibrary.GetClassDisplayName` (`GameplayStatics.GetObjectClass` self))) true true (struct :`R` 1.0 :`G` 0.05448 :`B` 0.001821 :`A` 1.0) 5.0)
  (`/Game/Core/Game/BP_GameState.RemoveState` (`/Game/Core/Common/Helpers/BFL_Getters.GetMTGameState`) self)
  (`self.Exit`))

(fn `Enter`)

(fn `Exit`)

(fn `Tick`)