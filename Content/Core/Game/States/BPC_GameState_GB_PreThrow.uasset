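; Game state component for the pre-throw phase that sets up the HUD and player input before a throw.
; On begin play it clears the CommonUI game stack, then after a short delay pushes the pre-throw HUD.
; It then shows the quick throw button and run HUD and reactivates controller inputs, which only happens if the pushed widget casts successfully.
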(event `self.ReceiveBeginPlay`
  (`/Game/Core/UI/CW_MainStack.RemoveGameStack` (`/Game/Core/Common/Helpers/BFL_Getters.GetCWMainStack`))
  (`KismetSystemLibrary.Delay` 0.5)
  (`/Game/Core/UI/CW_MainStack.PushGameStack` (`/Game/Core/Common/Helpers/BFL_Getters.GetCWMainStack`) "/Game/Core/UI/CW_PreThrowHUD.CW_PreThrowHUD_C")
  (bind _ascw_pre_throw_hud (cast `/Game/Core/UI/CW_PreThrowHUD` (`CommonActivatableWidgetContainerBase.GetActiveWidget` (`/Game/Core/UI/CW_MainStack.GameStack` (`/Game/Core/Common/Helpers/BFL_Getters.GetCWMainStack`)))))
  (`Widget.SetVisibility` (`/Game/Core/UI/CW_PreThrowHUD.ButtonQuickThrow` _ascw_pre_throw_hud) "Visible")
  (`Widget.SetVisibility` (`/Game/Core/UI/CW_MainStack.CW_RunHUD` (`/Game/Core/Common/Helpers/BFL_Getters.GetCWMainStack`)) "SelfHitTestInvisible")
  (`/Game/Core/Player/BP_PlayerController_Game.ReactivateInputs` (`/Game/Core/Common/Helpers/BFL_Getters.GetMTGameController`)))