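; BPC_GameState_Idle is the game state component for the idle phase, setting up the player when that state begins.
; On BeginPlay it checks the game state's previous state.
; After a GB round end it activates the crosshair, switches to the default camera, shows the showcase dice and processes the run data save.
; From any other state it has the player character enter the house.
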(event `self.ReceiveBeginPlay`
  (if (== (`/Game/Core/Game/BP_GameState.PreviousState` (`/Game/Core/Common/Helpers/BFL_Getters.GetMTGameState`)) "/Game/Core/Game/States/BPC_GameState_GB_RoundEnd.BPC_GameState_GB_RoundEnd_C")
    (`/Game/Core/Player/BP_PlayerCharacter.ActivatePlayerCrosshair` (`/Game/Core/Common/Helpers/BFL_Getters.GetMTPlayerCharacter`))
    (`/Game/Core/Player/BP_PlayerController_Game.SwitchToDefaultCamera` (`/Game/Core/Common/Helpers/BFL_Getters.GetMTGameController`))
    (`/Game/Core/Game/BP_GameState.ShowShowcaseDices` (`/Game/Core/Common/Helpers/BFL_Getters.GetMTGameState`))
    (`/Game/Core/Player/BP_PlayerCharacter.ProcessRunDataSave` (`/Game/Core/Common/Helpers/BFL_Getters.GetMTPlayerCharacter`))
    (else
      (`/Game/Core/Player/BP_PlayerCharacter.EnterHouse` (`/Game/Core/Common/Helpers/BFL_Getters.GetMTPlayerCharacter`)))))